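; Bomb bonus actor that produces an expanding blast at the player cube, destroying any BP_SpawningCube that overlaps its collision box.
; On BeginPlay it plays a sound and starts a looping timer that drives the explosion.
; Each tick of that timer snaps the bomb mesh to the player cube and scales the actor from a float curve, until the accumulated time reaches a hardcoded limit and the bomb destroys itself.
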(event OnComponentBeginOverlap(BombCollisionBox)
  (params (OverlappedComponent :type Primitive%20Component%20Object%20Reference) (OtherActor :type Actor%20Object%20Reference) (OtherComp :type Primitive%20Component%20Object%20Reference) (OtherBodyIndex :type Integer) (bFromSweep :type Boolean) (SweepResult :type Hit%20Result%20Structure%20%28by%20ref%29))
  (bind _asbp_spawning_cube (Utilities|Casting|CastToBP_SpawningCube OtherActor))
  (Actor|DestroyActor _asbp_spawning_cube))

(event Custom|Explosion
  ;[1 1 1] Set BombBonus location to complete the animation at the BP_Player location
  (Transformation|SetWorldLocation (Variables|Components|GetBombStaticMesh) (Transformation|GetWorldLocation (Variables|/Game/Gameplay/Blueprints/Player/BP_Player.BP_Player_C|GetPlayerCube (.AsBP%20Player (Utilities|Casting|CastToBP_Player (Game|Player|GetPlayerPawn 0))))) false false)
  ;[1 1 1] Set BombBomus scale
  (Transformation|SetActorScale3D (Math|Vector|MakeVector (Math|Curves|GetFloatValue (Variables|System|GetExplosionCurve) (Variables|System|GetInTime)) (Math|Curves|GetFloatValue (Variables|System|GetExplosionCurve) (Variables|System|GetInTime)) (Math|Curves|GetFloatValue (Variables|System|GetExplosionCurve) (Variables|System|GetInTime))))
  ;[1 1 1] Increase inTime
  (bind _output_get (Variables|System|SetInTime (+ (Variables|System|GetInTime) (Variables|System|GetTimerRate))))
  (if (>= _output_get 2.2)
    (Actor|DestroyActor)))

(event EventBeginPlay
  (Audio|PlaySound2D (Variables|System|GetInitialSound) 1.0 1.0 0.0 0 0)
  (Utilities|Time|SetTimerbyEvent (delegate Custom|Explosion) (Variables|System|GetTimerRate) true))

(fn ConstructionScript)