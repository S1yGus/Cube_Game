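; Player cube for a cube-collecting game, snapping left and right between target points from a random start.
; Overlapped cubes set its material and sound, drive score, time and speed through BPCTimeScoreSpeed, then get destroyed.
; Repeated same-type pickups build a capped multiplier, which also turns negative scores positive above one.
; Bonus cubes give BPCBonus a random missile, shield or bomb, spawned at the player cube on use.
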(event OnComponentBeginOverlap(PlayerCollisionBox)
  (params (OverlappedComponent :type Primitive%20Component%20Object%20Reference) (OtherActor :type Actor%20Object%20Reference) (OtherComp :type Primitive%20Component%20Object%20Reference) (OtherBodyIndex :type Integer) (bFromSweep :type Boolean) (SweepResult :type Hit%20Result%20Structure%20%28by%20ref%29))
  ;[1 1 1] Get cube
  (bind _asbp_base_cube (Utilities|Casting|CastToBP_BaseCube OtherActor))
  (Variables|System|SetOverlapedCube _asbp_base_cube)
  (System|GetCube)
  ;;[1 1 1] Set normal material after get cube
  (Utilities|FlowControl|Delay (Variables|Settings|Materials|GetGetCubeChangeMaterialTime))
  (Rendering|Material|SetMaterial (Variables|Default|GetPlayerCube) 0 (Variables|Settings|Materials|GetPlayerNormalMaterial)))

(event EventBeginPlay
  (System|Initialization)
  (Control|SetPosition))

(event Input|ActionEvents|InputActionLeft
  (params (Key :type Key%20Structure))
  ;[1 1 1] Control
  (:Pressed
    (Control|PositionLeft)
    (Control|SetPosition)))

(event Input|ActionEvents|InputActionRight
  (params (Key :type Key%20Structure))
  ;[1 1 1] Control
  (:Pressed
    (Control|PositionRight)
    (Control|SetPosition)))

(event Input|ActionEvents|InputActionQuit
  (params (Key :type Key%20Structure))
  (:Pressed
    (Game|QuitGame 0 "Quit" false)))

(event Input|ActionEvents|InputActionUseBonus
  (params (Key :type Key%20Structure))
  ;[1 1 1] Control
  (:Pressed
    (System|UseCurrentBonus)))

(fn ConstructionScript)

(fn PositionLeft
  (bind _result (Math|Integer|DecrementInt (Variables|System|Control|GetPosition))
    (:%20%20
      (if (< _result 0)
        (Variables|System|Control|SetPosition 0)
        (Audio|PlaySound2D (Variables|Settings|Sound|GetOutOfPosition) 1.0 1.0 0.0 0 0))
      (return))))

(fn PositionRight
  (bind _result (Math|Integer|IncrementInt (Variables|System|Control|GetPosition))
    (:%20%20
      (if (> _result (Variables|System|Control|GetPositionsAmount))
        (Variables|System|Control|SetPosition (Variables|System|Control|GetPositionsAmount))
        (Audio|PlaySound2D (Variables|Settings|Sound|GetOutOfPosition) 1.0 1.0 0.0 0 0))
      (return))))

(fn GetPosition
  ;[1 1 1] Get the position of the selected target point on the field
  (return (+ (Transformation|GetActorLocation (Utilities|Array|Get(acopy) (Variables|Settings|GetPlaerPositionsPoints) (Variables|System|Control|GetPosition))) (Variables|System|Control|GetPossitonZOffset))))

(fn SetPosition
  (Transformation|SetWorldLocation (Variables|Default|GetPlayerCube) (Control|GetPosition) false false)
  (return))

(fn GetCube
  (bind _output_get (LocalVariables|SetL_OverlapedCubeType (Default|GetCubeType (Variables|System|GetOverlapedCube))))
  ;[1 1 1] Multiply count change
  (if (Utilities|Enum|Equal(Enum) _output_get (Variables|System|Myltiply|GetPreviousCubeType))
    (bind _result (Math|Integer|IncrementInt (Variables|System|Myltiply|GetMultiplyCount))
      (:%20%20
        (if (> _result (Variables|System|Myltiply|GetMaxMultiplyCount))
          (Variables|System|Myltiply|SetMultiplyCount (Variables|System|Myltiply|GetMaxMultiplyCount)))))
    (else
      (Variables|System|Myltiply|SetMultiplyCount 0)))
  (Variables|System|Myltiply|SetPreviousCubeType (LocalVariables|GetL_OverlapedCubeType))
  ;[1 1 1] Set player material
  (Rendering|Material|SetMaterial (Variables|Default|GetPlayerCube) 0 (Utilities|Select :Index (LocalVariables|GetL_OverlapedCubeType) :NewEnumerator0 (Variables|Settings|Materials|GetGetGoodCubeMaterial) :NewEnumerator1 (Variables|Settings|Materials|GetGetBadCubeMaterial) :NewEnumerator2 (Variables|Settings|Materials|GetGetScoreCubeMaterial) :NewEnumerator3 (Variables|Settings|Materials|GetGetTimeCubeMaterial) :NewEnumerator4 (Variables|Settings|Materials|GetGetBonusCubeMaterial) :NewEnumerator5 (Variables|Settings|Materials|GetGetSpeedCubeMaterial) :NewEnumerator6 0))
  ;[1 1 1] Play take cube sound
  (Audio|PlaySound2D (Utilities|Select :Index (LocalVariables|GetL_OverlapedCubeType) :NewEnumerator0 (Variables|Settings|Sound|GetGetGoodCubeSound) :NewEnumerator1 (Variables|Settings|Sound|GetGetBadCubeSound) :NewEnumerator2 (Variables|Settings|Sound|GetGetScoreCubeSound) :NewEnumerator3 (Variables|Settings|Sound|GetGetTimeCubeSound) :NewEnumerator4 (Variables|Settings|Sound|GetGetBonusCubeSound) :NewEnumerator5 (Variables|Settings|Sound|GetGetSpeedCubeSound) :NewEnumerator6 0) 1.0 1.0 0.0 0 0)
  (switch Utilities|FlowControl|Switch|SwitchonEnum_CubesTypes (LocalVariables|GetL_OverlapedCubeType)
    (:NewEnumerator0
      _)
    (:NewEnumerator1
      _)
    (:NewEnumerator2
      _)
    (:NewEnumerator3
      _)
    (:NewEnumerator4
      ;[1 1 1] Take random bonus from bonus cube
      (Default|ChangeBonus (Variables|Default|GetBPC_Bonus) (Utilities|Select :Index (Math|Random|RandomIntegerinRange 0 2) :Option%200 "NewEnumerator0" :Option%201 "NewEnumerator1" :Option%202 "NewEnumerator2")))
    (:NewEnumerator5
      ;[1 1 1] Decrease by speed cube
      (Default|ChangeSpeed (Variables|Default|GetBPC_TimeScoreSpeed) false)))
  ;[1 1 1] Change score
  (Variables|System|SetCurrentCubeScore (select (> (Variables|System|Myltiply|GetMultiplyCount) 1) (Math|Integer|Absolute(Integer) (Utilities|Select :Index (LocalVariables|GetL_OverlapedCubeType) :NewEnumerator0 (Variables|System|ScoreChange|GetScoreChangeByGoodCube) :NewEnumerator1 (Variables|System|ScoreChange|GetScoreChangeByBadCube) :NewEnumerator2 (Variables|System|ScoreChange|GetScoreChangeByScoreCube) :NewEnumerator3 (Variables|System|ScoreChange|GetScoreChangeByTimeCube) :NewEnumerator4 (Variables|System|ScoreChange|GetScoreChangeByBonusCube) :NewEnumerator5 (Variables|System|ScoreChange|GetScoreChangeBySpeedCube) :NewEnumerator6 0)) (Utilities|Select :Index (LocalVariables|GetL_OverlapedCubeType) :NewEnumerator0 (Variables|System|ScoreChange|GetScoreChangeByGoodCube) :NewEnumerator1 (Variables|System|ScoreChange|GetScoreChangeByBadCube) :NewEnumerator2 (Variables|System|ScoreChange|GetScoreChangeByScoreCube) :NewEnumerator3 (Variables|System|ScoreChange|GetScoreChangeByTimeCube) :NewEnumerator4 (Variables|System|ScoreChange|GetScoreChangeByBonusCube) :NewEnumerator5 (Variables|System|ScoreChange|GetScoreChangeBySpeedCube) :NewEnumerator6 0)))
  ;;[1 0.2865 0.2865] Call ED_MultiplyChange when CurrentCubeScore already known
  (Default|CallEDMultiplyChange)
  (Default|ChangeScore (Variables|Default|GetBPC_TimeScoreSpeed) (* (Variables|System|GetCurrentCubeScore) (select (> (Variables|System|Myltiply|GetMultiplyCount) 1) (Variables|System|Myltiply|GetMultiplyCount) 1)))
  ;[1 1 1] Turn on ScoreWidget
  (Default|ChangeText (Variables|UI|GetW_ScoreInGame) (Variables|System|GetCurrentCubeScore) (Variables|System|Myltiply|GetMultiplyCount))
  ;[1 1 1] Change time
  (Default|ChangeTime (Variables|Default|GetBPC_TimeScoreSpeed) (Utilities|Select :Index (LocalVariables|GetL_OverlapedCubeType) :NewEnumerator0 (Variables|System|TimeChange|GetTimeChangeByGoodCube) :NewEnumerator1 (Variables|System|TimeChange|GetTimeChangeByBadCube) :NewEnumerator2 (Variables|System|TimeChange|GetTimeChangeByScoreCube) :NewEnumerator3 (Variables|System|TimeChange|GetTimeChangeByTimeCube) :NewEnumerator4 (Variables|System|TimeChange|GetTimeChangeByBonusCube) :NewEnumerator5 (Variables|System|TimeChange|GetTimeChangeBySpeedCube) :NewEnumerator6 0))
  (Actor|DestroyActor (Variables|System|GetOverlapedCube))
  (return))

(fn SetTimeChangebyCubesValues
  (params (TimeChangeByGoodCube :type Integer) (TimeChangeByBadCube :type Integer) (TimeChangeByScoreCube :type Integer) (TimeChangeByTimeCube :type Integer) (TimeChangeByBonusCube :type Integer) (TimeChangeBySpeedCube :type Integer))
  (Variables|System|TimeChange|SetTimeChangeByGoodCube TimeChangeByGoodCube)
  (Variables|System|TimeChange|SetTimeChangeByBadCube TimeChangeByBadCube)
  (Variables|System|TimeChange|SetTimeChangeByScoreCube TimeChangeByScoreCube)
  (Variables|System|TimeChange|SetTimeChangeByTimeCube TimeChangeByTimeCube)
  (Variables|System|TimeChange|SetTimeChangeByBonusCube TimeChangeByBonusCube)
  (Variables|System|TimeChange|SetTimeChangeBySpeedCube TimeChangeBySpeedCube)
  (return))

(fn SetScoreChanbebyCubesValues
  (params (ScoreChangeByGoodCube :type Integer) (ScoreChangeByBadCube :type Integer) (ScoreChangeByScoreCube :type Integer) (ScoreChangeByTimeCube :type Integer) (ScoreChangeByBonusCube :type Integer) (ScoreChangeBySpeedCube :type Integer))
  (Variables|System|ScoreChange|SetScoreChangeByGoodCube ScoreChangeByGoodCube)
  (Variables|System|ScoreChange|SetScoreChangeByBadCube ScoreChangeByBadCube)
  (Variables|System|ScoreChange|SetScoreChangeByScoreCube ScoreChangeByScoreCube)
  (Variables|System|ScoreChange|SetScoreChangeByTimeCube ScoreChangeByTimeCube)
  (Variables|System|ScoreChange|SetScoreChangeByBonusCube ScoreChangeByBonusCube)
  (Variables|System|ScoreChange|SetScoreChangeBySpeedCube ScoreChangeBySpeedCube)
  (return))

(fn UseCurrentBonus
  (Game|SpawnActorfromClass (Utilities|Select :Index (Default|GetCurrentBonus (Variables|Default|GetBPC_Bonus)) :NewEnumerator3 0 :NewEnumerator0 "/Game/Gameplay/Blueprints/Bonuses/BP_MissileBonus.BP_MissileBonus_C" :NewEnumerator1 "/Game/Gameplay/Blueprints/Bonuses/BP_ShieldBonus.BP_ShieldBonus_C" :NewEnumerator2 "/Game/Gameplay/Blueprints/Bonuses/BP_BombBonus.BP_BombBonus_C") (Transformation|GetWorldTransform (Variables|Default|GetPlayerCube)) "Undefined" 0 0)
  (Default|ChangeBonus (Variables|Default|GetBPC_Bonus) "NewEnumerator3"))

(fn Initialization
  ;[1 1 1] Set number of positions and random start position
  (bind _output_get (Variables|System|Control|SetPositionsAmount (- (Utilities|Array|Length (Variables|Settings|GetPlaerPositionsPoints)) 1)))
  (Variables|System|Control|SetPosition (Math|Random|RandomIntegerinRange 0 _output_get))
  ;[1 1 1] Get W_ScoreInGame varible
  (Variables|UI|SetW_ScoreInGame (.AsW%20Score%20in%20Game (Utilities|Casting|CastToW_ScoreInGame (UserInterface|GetWidget (Variables|Default|GetScoreWidget)))))
  (return))

(fn GetMultiplyInfo
  (return (Variables|System|Myltiply|GetMultiplyCount) (!= (Variables|System|GetCurrentCubeScore) 0) (Variables|System|Myltiply|GetPreviousCubeType)))

(fn SetScoretoSpeedUp
  (params (ScoreToSpeedUp :type Integer))
  (Default|SetScoretoSpeedUp (Variables|Default|GetBPC_TimeScoreSpeed) ScoreToSpeedUp)
  (return))