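; Player component that tracks remaining time, score and movement speed, broadcasting changes through event dispatchers.
; A looping one-second timer counts seconds down, warns when time runs low and triggers game over with a sound at zero.
; Score accumulates toward a threshold that raises speed, and a negative score also ends the game.
; Speed changes by a fixed step, clamped to a minimum, while tracking the number of speed-ups.
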(event Custom|Countdown
  (if (<= (Variables|System|Time|GetSeconds) (Variables|Settings|Time|GetLowTimeWarningSeconds))
    (Default|CallEDLowTime))
  (if (== (Variables|System|Time|GetSeconds) 0)
    (Audio|PlaySound2D (Variables|Settings|Sound|GetGameOverSound) 1.0 1.0 0.0 0 0)
    (Default|CallEDGameOver)
    (else
      (Math|Integer|DecrementInt (Variables|System|Time|GetSeconds)
        (:%20%20
          (Default|CallEDChangeTime))))))

(event EventBeginPlay
  (Utilities|Time|SetTimerbyEvent (delegate Custom|Countdown) 1.0 true))

(fn ChangeSpeed
  (params (IncreaseSpeed :type Boolean))
  (if IncreaseSpeed
    ;[1 1 1] Increase speed
    (Variables|System|Speed|SetSpeed (+ (Variables|System|Speed|GetSpeed) (Variables|Settings|Speed|GetChangeSpeedValue)))
    (Math|Integer|IncrementInt (Variables|System|Speed|GetSpeedCount)
      (:%20%20
        _))
    (else
      ;[1 1 1] Decrease speed
      (Variables|System|Speed|SetSpeed (Math|Float|Max(Float) (- (Variables|System|Speed|GetSpeed) (Variables|Settings|Speed|GetChangeSpeedValue)) (Variables|Settings|Speed|GetMinSpeed)))
      (Variables|System|Speed|SetSpeedCount (Math|Integer|Max(Integer) (- (Variables|System|Speed|GetSpeedCount) 1)))))
  (Default|CallEDChangeSpeed)
  (return))

(fn ChangeScore
  (params (AddScore :type Integer))
  ;[1 1 1] Accumulate speed up score
  (Variables|System|Score|SetSpeedUpScore (+ AddScore (Variables|System|Score|GetSpeedUpScore)))
  ;[1 1 1] Accumulate score
  (bind _output_get (Variables|System|Score|SetScore (+ AddScore (Variables|System|Score|GetScore))))
  (Default|CallEDChangeScore)
  (if (< _output_get 0)
    (Audio|PlaySound2D (Variables|Settings|Sound|GetGameOverSound) 1.0 1.0 0.0 0 0)
    (Default|CallEDGameOver)
    (return)
    (else
      ;[1 1 1] If SpeedUpScore > ScoreToSpeedUp - 1, then increase speed and set new SpeedUpScore
      (if (> (Variables|System|Score|GetSpeedUpScore) (- (Variables|Settings|Score|GetScoreToSpeedUp) 1))
        (Variables|System|Score|SetSpeedUpScore (Math|Integer|%(Integer) (Variables|System|Score|GetScore) (Variables|Settings|Score|GetScoreToSpeedUp)))
        (System|ChangeSpeed true)
        (return)))))

(fn ChangeTime
  (params (AddSeconds :type Integer))
  (Variables|System|Time|SetSeconds (Math|Integer|Max(Integer) (+ AddSeconds (Variables|System|Time|GetSeconds))))
  (Default|CallEDChangeTime)
  (return))

(fn GetSpeed
  (return (Variables|System|Speed|GetSpeed)))

(fn GetScore
  (return (Variables|System|Score|GetScore)))

(fn GetTime
  (return (Variables|System|Time|GetSeconds)))

(fn SetScoretoSpeedUp
  (params (ScoreToSpeedUp :type Integer))
  (Variables|Settings|Score|SetScoreToSpeedUp ScoreToSpeedUp)
  (return))

(fn GetSpeedCount
  (return (Variables|System|Speed|GetSpeedCount)))