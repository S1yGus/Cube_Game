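; Player component that holds the current bonus: None, Missile, Shield or Bomb.
; ChangeBonus stores the new bonus, writes its matching colour to the FieldColour parameter of the MPC_Field material parameter collection, then fires the bonus-change event dispatcher.
; GetCurrentBonus returns the stored value.
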(fn ChangeBonus
  (params (NewBonus :type Emun_Bonuses%20Enum :default "NewEnumerator3"))
  (bind _output_get (Variables|System|SetCurrentBonus NewBonus))
  ;[1 1 1] Set field colour
  (Rendering|Material|SetVectorParameterValue "/Game/Materials/MPC_Field.MPC_Field" "FieldColour" (Utilities|Select :Index _output_get :NewEnumerator3 (Variables|Settings|Colours|GetColourNone) :NewEnumerator0 (Variables|Settings|Colours|GetColourMissile) :NewEnumerator1 (Variables|Settings|Colours|GetColourShild) :NewEnumerator2 (Variables|Settings|Colours|GetColourBomb)) :!class /Script/Engine.KismetMaterialLibrary)
  (Default|CallEDChageBonus)
  (return))

(fn GetCurrentBonus
  (return (Variables|System|GetCurrentBonus)))