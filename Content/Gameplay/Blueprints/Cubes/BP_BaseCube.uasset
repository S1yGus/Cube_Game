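; BP_BaseCube is a base cube actor that moves along its local X axis at a game-driven speed.
; On BeginPlay it reads Speed from the player pawn's BPCTimeScoreSpeed component and applies it as ProjectileMovement velocity.
; It also binds to that component's speed-change event dispatcher.
; A getter exposes its CubeType.
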(event EventBeginPlay
  (EventDispatchers|BindEventtoEDChangeSpeed (System|GetBPCTimeScoreSpeed) (EventDispatchers|CreateEvent :!event SetSpeed))
  (System|SetSpeed)
  (System|Moving))

(fn ConstructionScript)

(fn SetSpeed
  (Variables|System|SetSpeed (Default|GetSpeed (System|GetBPCTimeScoreSpeed)))
  (return))

(fn GetBPCTimeScoreSpeed
  (return (Variables|/Game/Gameplay/Blueprints/Player/BP_Player.BP_Player_C|GetBPC_TimeScoreSpeed (.AsBP%20Player (Utilities|Casting|CastToBP_Player (Game|Player|GetPlayerPawn 0))))))

(fn GetCubeType
  (return (Variables|System|GetCubeType)))

(fn Moving
  (Game|Components|ProjectileMovement|SetVelocityinLocalSpace (Variables|Default|GetProjectileMovement) (Math|Vector|MakeVector (Variables|System|GetSpeed) 0.0 0.0))
  (return))