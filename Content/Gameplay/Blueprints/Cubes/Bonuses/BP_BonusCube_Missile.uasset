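; Missile variant of a bonus cube, a child Blueprint that travels as a projectile.
; On BeginPlay it runs the parent logic, then Moving sets the ProjectileMovement velocity along local Z at MissileSpeed, so its spawn rotation determines the flight direction.
; The OverlapEnding event calls Destructor, and the construction script only runs the parent's.
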(event EventBeginPlay
  (|CallParentFunction)
  (CallFunction|Moving))

(event EventOverlapEnding
  (CallFunction|Destructor))

(fn ConstructionScript
  (|CallParentFunction))

(fn Moving
  (Game|Components|ProjectileMovement|SetVelocityinLocalSpace (Variables|Default|GetProjectileMovement) (Math|Vector|MakeVector 0.0 0.0 (Variables|System|GetMissileSpeed)))
  (return))