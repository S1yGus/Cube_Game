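; Base Blueprint for bonus cubes, which react when they collide with a spawning cube.
; The Constructor event runs the parent logic and plays an initial 2D sound.
; A collision box overlap with a BP_SpawningCube calls that cube's Destructor, plays a hit sound, then fires OverlapEnding.
; OverlapEnding is left empty here as a hook for bonus-specific behavior.
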(event OnComponentBeginOverlap(CollisionBox)
  (params (OverlappedComponent :type Primitive%20Component%20Object%20Reference) (OtherActor :type Actor%20Object%20Reference) (OtherComp :type Primitive%20Component%20Object%20Reference) (OtherBodyIndex :type Integer) (bFromSweep :type Boolean) (SweepResult :type Hit%20Result%20Structure%20%28by%20ref%29))
  (bind _asbp_spawning_cube (Utilities|Casting|CastToBP_SpawningCube OtherActor))
  (Default|Destructor _asbp_spawning_cube)
  (Audio|PlaySound2D (Variables|System|Sound|GetHitSound) 1.0 1.0 0.0 0 0)
  (CallFunction|OverlapEnding))

(event Custom|OverlapEnding)

(event EventBeginPlay
  (|CallParentFunction))

(event EventConstructor
  (|CallParentFunction)
  (Audio|PlaySound2D (Variables|System|Sound|GetInitialSound) 1.0 1.0 0.0 0 0))

(fn ConstructionScript
  (|CallParentFunction))