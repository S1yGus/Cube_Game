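; BP_SpawningCube is a cube that moves along its local X axis via projectile movement at a game-wide speed.
; On BeginPlay it reads Speed from the player's BPC_TimeScoreSpeed component, binds to that component's speed-change dispatcher, and sets its velocity.
; Constructor and Destructor events extend the parent's, switching the mesh's collision between query-only and disabled.
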(event EventBeginPlay
  (|CallParentFunction)
  (EventDispatchers|BindEventtoEDChangeSpeed (System|GetBPCTimeScoreSpeed) (EventDispatchers|CreateEvent :!event SetSpeed))
  (System|SetSpeed)
  (System|Moving))

(event EventDestructor
  (|CallParentFunction)
  (Collision|SetCollisionEnabled (Variables|Default|GetCubeStaticMesh) "NoCollision"))

(event EventConstructor
  (|CallParentFunction)
  (Collision|SetCollisionEnabled (Variables|Default|GetCubeStaticMesh) "QueryOnly"))

(fn ConstructionScript)

(fn SetSpeed
  (Variables|System|Movement|SetSpeed (Default|GetSpeed (System|GetBPCTimeScoreSpeed)))
  (return))

(fn GetBPCTimeScoreSpeed
  (return (Variables|/Game/Gameplay/Blueprints/Player/BP_Player.BP_Player_C|GetBPC_TimeScoreSpeed (.AsBP%20Player (Utilities|Casting|CastToBP_Player (Game|Player|GetPlayerPawn 0))))))

(fn Moving
  (Game|Components|ProjectileMovement|SetVelocityinLocalSpace (Variables|Default|GetProjectileMovement) (Math|Vector|MakeVector (Variables|System|Movement|GetSpeed) 0.0 0.0))
  (return))