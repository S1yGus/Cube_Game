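; Base UI cube actor that sets its mesh material and animates its uniform scale.
; BeginPlay applies the configured material, then Tick moves the current scale toward a target at a constant interpolation speed.
; The Destructor event sets the target scale to zero, waits briefly so the cube can shrink, then destroys the actor.
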(event Custom|Destructor
  ;[1 1 1] Destructor
  (Variables|System|SetScaleTarget 0.0)
  (Utilities|FlowControl|Delay 0.5)
  (Actor|DestroyActor))

(event EventTick
  (params (DeltaSeconds :type Float%20%28single-precision%29))
  ;[1 1 1] Sst scale
  (bind _output_get (Variables|System|SetCurrentScale (Math|Interpolation|FInterptoConstant (Variables|System|GetCurrentScale) (Variables|System|GetScaleTarget) DeltaSeconds (Variables|System|GetScaleChnageSpeed))))
  (Transformation|SetActorScale3D (Math|Vector|MakeVector _output_get _output_get _output_get)))

(event EventBeginPlay
  ;[1 1 1] Set material
  (Rendering|Material|SetMaterial (Variables|Default|GetMultiplyCubeStaticMesh) 0 (Variables|System|GetNewMaterial)))

(fn ConstructionScript)