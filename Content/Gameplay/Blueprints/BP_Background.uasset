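; BP_Background is an audio visualizer that animates a spawned grid of background cubes to music.
; Every fourth audio playback callback samples baked Synesthesia Constant-Q bands for the playing wave at the current time.
; Bands drive each cube's height and scale, the shared MPC_Cubes emissive pulse, and, every eleventh band, the height of BP_Game's UI cubes.
; A looping timer prints the average update rate.
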(event Custom|SpawnBackgroundCubes
  ;[1 1 1] Spawn matrix of cubes on background
  (for _index (range 0 (Variables|Settings|Background|GetRows))
    (for _index_2 (range 0 (Variables|Settings|Background|GetCols))
      (bind _returnvalue (Game|SpawnActorfromClass "/Game/Gameplay/Blueprints/Cubes/Background_Cubes/BP_BackgroundCube.BP_BackgroundCube_C" (Math|Transform|MakeTransform (Math|Vector|MakeVector (+ (Variables|Settings|Background|GetColsOffset) (* _index_2 (Variables|Settings|Background|GetDistanceBetweenCubes))) (+ (Variables|Settings|Background|GetRowsOffset) (* _index (Variables|Settings|Background|GetDistanceBetweenCubes))) (Variables|Settings|Background|GetSpawnCubesLocationZ)) "0, 0, 0" "1,1,1") "Undefined" 0 0))
      (Utilities|Array|Add (Variables|System|GetCubes) _returnvalue))))

(event Custom|Timer
  (Math|Float|IncrementFloat (Variables|Default|GetY)
    (:%20%20
      (Development|PrintString (Utilities|String|ToString(Float) (/ (Variables|Default|GetZ) (Variables|Default|GetY)))))))

(event EventBeginPlay
  (CallFunction|SpawnBackgroundCubes)
  (CallFunction|Initialization)
  (EventDispatchers|BindEventtoOnAudioPlaybackPercent (Variables|Default|GetAudio) (EventDispatchers|CreateEvent :!event Synesthesia))
  (Audio|Components|Audio|Play (Variables|Default|GetAudio) 0.0)
  (Utilities|Time|SetTimerbyEvent (delegate Custom|Timer) 1.0 true))

(fn ConstructionScript)

(fn Synesthesia
  (params (PlayingSoundWave :type Sound%20Wave%20Object%20Reference) (PlaybackPercent :type Float%20%28single-precision%29))
  (bind _synesthesiamap (Variables|Settings|GetSynesthesiaMap))
  (bind _bp_game (Variables|System|GetBP_Game))
  (bind _spawned_ui_bonuscube (Default|GetSpawnedUIBonusCube _bp_game))
  (bind (_value _returnvalue) (Utilities|Map|Find _synesthesiamap PlayingSoundWave))
  (bind _result (Math|Float|IncrementFloat (Variables|Default|GetX))
    (:%20%20
      (if (== (Math|Float|%(Float) _result 4.0) 0.0)
        (Math|Float|IncrementFloat (Variables|Default|GetZ)
          (:%20%20
            ;[1 1 1] If there is synesthesia asset for current wave
            (if _returnvalue
              ;[1 1 1] Checking for UI cubes
              (LocalVariables|SetL_SpawnedUIMultiplyCubes (Default|GetSpawnedUIMultiplyCubes _bp_game))
              (Utilities|IsValid _spawned_ui_bonuscube
                (:Is%20Valid
                  (Utilities|Array|Add (LocalVariables|GetL_SpawnedUIMultiplyCubes) _spawned_ui_bonuscube))
                (:Is%20Not%20Valid
                  _))
              (for (_array_element _array_index) (Class|ConstantQNRT|GetNormalizedChannelConstantQatTime _value (* (Variables|/Script/Engine.SoundBase|GetDuration PlayingSoundWave) PlaybackPercent))
                (LocalVariables|SetL_CurrentBand _array_element)
                (Utilities|IsValid (Utilities|Array|Get(acopy) (Variables|System|GetCubes) _array_index)
                  (:Is%20Valid
                    (LocalVariables|SetL_CurrentCube (Utilities|Array|Get(acopy) (Variables|System|GetCubes) _array_index))
                    (if (== (Math|Integer|%(Integer) _array_index 11) 0)
                      ;[1 1 1] If UI cubes is valids set z location for them depending on the synesthesia band
                      (Utilities|IsValid (Utilities|Array|Get(acopy) (LocalVariables|GetL_SpawnedUIMultiplyCubes) (LocalVariables|GetL_UICubesCounter))
                        (:Is%20Valid
                          (Transformation|SetActorLocation (Utilities|Array|Get(acopy) (LocalVariables|GetL_SpawnedUIMultiplyCubes) (LocalVariables|GetL_UICubesCounter)) (Math|Vector|MakeVector (.x (Transformation|GetActorLocation (Utilities|Array|Get(acopy) (LocalVariables|GetL_SpawnedUIMultiplyCubes) (LocalVariables|GetL_UICubesCounter)))) (.y (Transformation|GetActorLocation (Utilities|Array|Get(acopy) (LocalVariables|GetL_SpawnedUIMultiplyCubes) (LocalVariables|GetL_UICubesCounter)))) (* (Variables|Settings|UI|GetUICubesMaxAmplitude) (LocalVariables|GetL_CurrentBand))) false false)
                          (Math|Integer|IncrementInt (LocalVariables|GetL_UICubesCounter)
                            (:%20%20
                              _)))
                        (:Is%20Not%20Valid
                          _)))
                    ;[1 1 1] Set current background cube z location depending on the synesthesia band
                    (Transformation|SetActorLocation (LocalVariables|GetL_CurrentCube) (Math|Vector|MakeVector (.x (Transformation|GetActorLocation (LocalVariables|GetL_CurrentCube))) (.y (Transformation|GetActorLocation (LocalVariables|GetL_CurrentCube))) (+ (* (Variables|Settings|Background|GetCubesMaxAmplitude) (LocalVariables|GetL_CurrentBand)) (Variables|Settings|Background|GetSpawnCubesLocationZ))) false false)
                    ;[1 1 1] Set current background cube scale depending on the synesthesia band
                    (Transformation|SetActorScale3D (LocalVariables|GetL_CurrentCube) (Math|Vector|MakeVector (* (LocalVariables|GetL_CurrentBand) (Variables|Settings|Background|GetCubesMaxScale)) (* (LocalVariables|GetL_CurrentBand) (Variables|Settings|Background|GetCubesMaxScale)) (* (LocalVariables|GetL_CurrentBand) (Variables|Settings|Background|GetCubesMaxScale))))
                    ;[1 1 1] Set cube materials emissive pulse depending on the synesthesia band
                    (Rendering|Material|SetScalarParameterValue "/Game/Materials/MPC_Cubes.MPC_Cubes" "EmissivePulse" (* (Variables|Settings|GetCubesMaxEmissivePower) (LocalVariables|GetL_CurrentBand)) :!class /Script/Engine.KismetMaterialLibrary))
                  (:Is%20Not%20Valid
                    (return))))
              (return)
              (else
                (return)))))
        (else
          (return))))))

(fn Initialization
  (Audio|Components|Audio|SetSound (Variables|Default|GetAudio) (Variables|Settings|GetSound))
  (bind _returnvalue (Actor|GetActorOfClass "/Game/Gameplay/Blueprints/BP_Game.BP_Game_C"))
  (Utilities|IsValid _returnvalue
    (:Is%20Valid
      (Variables|System|SetBP_Game _returnvalue)
      (return))
    (:Is%20Not%20Valid
      (return))))