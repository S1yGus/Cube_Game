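; BP_MainMenuCamera is the main menu camera, which adapts its framing to the aspect ratio held by BP_GameInstance.
; On BeginPlay it binds to the game instance's aspect-ratio-changed dispatcher.
; ChangeAspectRatio constrains the camera to that ratio and selects a separate field of view for 16:9 or 21:9.
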(event EventBeginPlay
  (EventDispatchers|BindEventtoEDChangedAspectRatio (System|GetGameInstance) (EventDispatchers|CreateEvent :!event ChangeAspectRatio)))

(fn ConstructionScript)

(fn ChangeAspectRatio
  (bind _bp_gameinstance (System|GetGameInstance))
  (bind _camera (Variables|Default|GetCamera))
  (Class|CameraComponent|SetConstraintAspectRatio _camera true)
  (Class|CameraComponent|SetAspectRatio _camera (Default|GetAspectRatio _bp_gameinstance))
  (Camera|SetFieldOfView _camera (Utilities|Select :Index (Default|GetAspectRatioType _bp_gameinstance) :NewEnumerator0 (LocalVariables|GetL_16:9_FieldOfView) :NewEnumerator1 (LocalVariables|GetL_21:9_FieldOfView)))
  (return))

(fn GetGameInstance
  (return (.AsBP%20Game%20Instance (Utilities|Casting|CastToBP_GameInstance (Game|GetGameInstance)))))