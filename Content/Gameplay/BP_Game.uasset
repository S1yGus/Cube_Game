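; BP_Game is the gameplay manager that applies the chosen difficulty to spawning and player time, score and speed-up settings.
; A looping timer, with interval derived from cube spacing and player speed, drives cube spawning.
; SpawnCube picks weighted random types and recurses by chance up to a depth limit, using unique points per wave.
; Player multiplier and bonus change events drive the spawning and clearing of UI indicator cubes.
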(event Custom|SpawnMultiplyCube
  (bind _bp_player (Variables|System|GetBP_Player))
  (bind (_multiplycount _ischangescore _cubetype) (Default|GetMultiplyInfo _bp_player))
  ;[1 1 1] Multiply change
  (bind _output_get (Variables|System|Spawn|SetCurrentMultiplyCount _multiplycount))
  (if (== _output_get 0)
    (for _array_element (Variables|System|Spawn|GetSpawnedUI_MultiplyCubes)
      (Default|Destructor _array_element))
    (Utilities|Array|Clear (Variables|System|Spawn|GetSpawnedUI_MultiplyCubes))
    (CallFunction|SpawnMultiplyCubeReset)
    (elif _ischangescore
      ;;[1 1 1] If CurrentMultiplyCount == MaxMultiplyCount spawn cube only one times
      (if (== (Variables|System|Spawn|GetCurrentMultiplyCount) (Variables|System|GetMaxMultiplyCount))
        (Utilities|FlowControl|DoOnce false
          (:Completed
            _)))
      (bind _returnvalue (Game|SpawnActorfromClass "/Game/Gameplay/Cubes/BP_UI_MultipyCube.BP_UI_MultipyCube_C" (Transformation|GetActorTransform (Utilities|Array|Get(acopy) (Variables|Settings|GetMultiplyCubeSpawnPoints) (- (Variables|System|Spawn|GetCurrentMultiplyCount) 1))) "Undefined" 0 _cubetype 0))
      (Utilities|Array|Add (Variables|System|Spawn|GetSpawnedUI_MultiplyCubes) _returnvalue))))

(event Custom|SetSpawnTimer
  ;[1 1 1] Set cpawn cube timer
  (if (Utilities|Time|IsValidTimerHandle (Variables|System|Spawn|GetSpawnCubeTimer))
    (Utilities|Time|ClearandInvalidateTimerbyHandle (Variables|System|Spawn|GetSpawnCubeTimer)))
  (bind _returnvalue (Utilities|Time|SetTimerbyEvent (EventDispatchers|CreateEvent :!event SpawnCube) (System|GetTimerRate) true))
  (Variables|System|Spawn|SetSpawnCubeTimer _returnvalue))

(event Custom|SpawnMultiplyCubeReset
  ;[1 1 1] Multiply change
  ;;[1 1 1] If CurrentMultiplyCount == MaxMultiplyCount spawn cube only one times
  (Utilities|FlowControl|DoOnce false) ; enters at Reset
)

(event EventBeginPlay
  (System|Constructor)
  ;[1 1 1] Start spawn cube timer
  (EventDispatchers|BindEventtoEDChangeSpeed (Variables|/Game/Gameplay/Player/BP_Player.BP_Player_C|GetBPC_TimeScoreSpeed (Variables|System|GetBP_Player)) (EventDispatchers|CreateEvent :!event Custom|SetSpawnTimer))
  (CallFunction|SetSpawnTimer)
  ;[1 1 1] Bind event to ED_MultiplyChange
  (EventDispatchers|BindEventtoEDMultiplyChange (Variables|System|GetBP_Player) (EventDispatchers|CreateEvent :!event Custom|SpawnMultiplyCube))
  ;[1 1 1] Bind event to ED_ChangeBonus
  (EventDispatchers|BindEventtoEDChageBonus (Variables|/Game/Gameplay/Player/BP_Player.BP_Player_C|GetBPC_Bonus (Variables|System|GetBP_Player)) (EventDispatchers|CreateEvent :!event SpawnUIBonusCube)))

(fn ConstructionScript)

(fn SpawnCube
  ;[1 1 1] Current recursion count
  (Math|Integer|IncrementInt (Variables|System|Spawn|GetCurrentRecursionDepth)
    (:%20%20
      (if (<= (Variables|System|Spawn|GetCurrentRecursionDepth) (Variables|System|Spawn|GetMaxRecursionDepth))
        ;[1 1 1] Until get a unique spawn poin number
        (while (LocalVariables|GetL_NeedUniqueValue)
          ;[1 1 1] Get random spawn point number, if it already was used in this recursion cycle get another one
          (LocalVariables|SetL_CurrentRndomPointNumber (Math|Random|RandomIntegerinRange 0 (Variables|System|Spawn|GetSpawnPointsAmount)))
          (if (not (Utilities|Array|ContainsItem (Variables|System|Spawn|GetPreviousSpawnPointsNumbers) (LocalVariables|GetL_CurrentRndomPointNumber)))
            (LocalVariables|SetL_NeedUniqueValue false)))
        ;[1 1 1] Add new unique spawn point number to previous spawn points numbers
        (Utilities|Array|Add (Variables|System|Spawn|GetPreviousSpawnPointsNumbers) (LocalVariables|GetL_CurrentRndomPointNumber))
        ;[1 1 1] Spawn random cube
        (Game|SpawnActorfromClass "/Game/Gameplay/Cubes/BP_SpawningCube.BP_SpawningCube_C" (Transformation|GetActorTransform (Utilities|Array|Get(acopy) (Variables|Settings|GetCubeSpawnPonts) (LocalVariables|GetL_CurrentRndomPointNumber))) "Undefined" 0 (System|GetRandomCubeType) 0)
        ;[1 1 1] Chance to trigger recursion
        (if (Math|Random|RandomBoolwithWeight (Variables|System|Spawn|GetChanceToTriggerRecursion))
          (System|SpawnCube)
          (return)
          (else
            _)))
      ;[1 1 1] End recursion
      (Variables|System|Spawn|SetCurrentRecursionDepth 0)
      (Utilities|Array|Clear (Variables|System|Spawn|GetPreviousSpawnPointsNumbers))
      (return))))

(fn GetTimerRate
  (return (/ (Variables|System|GetDistanceBetweenCubes) (Default|GetSpeed (Variables|/Game/Gameplay/Player/BP_Player.BP_Player_C|GetBPC_TimeScoreSpeed (.AsBP%20Player (Utilities|Casting|CastToBP_Player (Game|Player|GetPlayerPawn 0))))))))

(fn SetTimeChangesbyCubeValues
  (Default|SetTimeChangebyCubesValues (Variables|System|GetBP_Player) (Variables|System|TimeChangesByCubes|GetTimeChangeByGoodCube) (Variables|System|TimeChangesbyCubes|GetTimeChangeByBadCube) (Variables|System|TimeChangesbyCubes|GetTimeChangeByScoreCube) (Variables|System|TimeChangesbyCubes|GetTimeChangeByTimeCube) (Variables|System|TimeChangesbyCubes|GetTimeChangeByBonusCube) (Variables|System|TimeChangesbyCubes|GetTimeChangeBySpeedCube))
  (return))

(fn SetScoreChangesbyCubeValues
  (Default|SetScoreChanbebyCubesValues (Variables|System|GetBP_Player) (Variables|System|ScoreChangeByCubes|GetScoreChangeByGoodCube) (Variables|System|ScoreChangebyCubes|GetScoreChangeByBadCube) (Variables|System|ScoreChangebyCubes|GetScoreChangeByScoreCube) (Variables|System|ScoreChangebyCubes|GetScoreChangeByTimeCube) (Variables|System|ScoreChangebyCubes|GetScoreChangeByBonusCube) (Variables|System|ScoreChangebyCubes|GetScoreChangeBySpeedCube))
  (return))

(fn GetRandomCubeType
  (bind _goodcube (Variables|System|Spawn|GetGoodCube))
  (bind _badcube (Variables|System|Spawn|GetBadCube))
  (return (Utilities|Select :Index (Math|Random|RandomIntegerinRange 0 15) :Option%200 _goodcube :Option%201 _goodcube :Option%202 _goodcube :Option%203 _goodcube :Option%204 _goodcube :Option%205 _badcube :Option%206 _badcube :Option%207 _badcube :Option%208 _badcube :Option%209 _badcube :Option%2010 (Variables|System|Spawn|GetScoreCube) :Option%2011 (Variables|System|Spawn|GetTimeCube) :Option%2012 (select (Math|Random|RandomBool) (Variables|System|Spawn|GetDifficultyTypeOption_01) (Variables|System|Spawn|GetBonusCube)) :Option%2013 (select (Math|Random|RandomBool) (Variables|System|Spawn|GetDifficultyTypeOption_02) (Variables|System|Spawn|GetSpeedCube)) :Option%2014 (Variables|System|Spawn|GetDifficultyTypeOption_01) :Option%2015 (Variables|System|Spawn|GetDifficultyTypeOption_02))))

(fn Constructor
  ;[1 1 1] Get difficulty from game instace
  (LocalVariables|SetL_Difficulty (Default|GetDifficulty (.AsBP%20Game%20Instance (Utilities|Casting|CastToBP_GameInstance (Game|GetGameInstance)))))
  ;[1 1 1] Set PB_Player
  (Variables|System|SetBP_Player (.AsBP%20Player (Utilities|Casting|CastToBP_Player (Game|Player|GetPlayerPawn 0))))
  ;[1 1 1] Set distance between cubes
  (Variables|System|SetDistanceBetweenCubes (Utilities|Select :Index (LocalVariables|GetL_Difficulty) :NewEnumerator0 (Variables|Settings|Difficulty|Easy|GetDistanceBetweenCubesEasy) :NewEnumerator1 (Variables|Settings|Difficulty|Medium|GetDistanceBetweenCubesMedium) :NewEnumerator2 (Variables|Settings|Difficulty|Hard|GetDistanceBetweenCubesHard)))
  ;[1 1 1] Set max recursion depth
  (Variables|System|Spawn|SetMaxRecursionDepth (Utilities|Select :Index (LocalVariables|GetL_Difficulty) :NewEnumerator0 (Variables|Settings|Difficulty|Easy|GetMaxRecursionDepthEasy) :NewEnumerator1 (Variables|Settings|Difficulty|Medium|GetMaxRecursionDepthMedium) :NewEnumerator2 (Variables|Settings|Difficulty|Hard|GetMaxRecursionDepthHard)))
  ;[1 1 1] Set spawn options
  (Variables|System|Spawn|SetDifficultyTypeOption_01 (Utilities|Select :Index (LocalVariables|GetL_Difficulty) :NewEnumerator0 (Variables|Settings|Difficulty|Easy|GetDifficultySpawnOption_01_Easy) :NewEnumerator1 (Variables|Settings|Difficulty|Medium|GetDifficultySpawnOption_01_Medium) :NewEnumerator2 (Variables|Settings|Difficulty|Hard|GetDifficultySpawnOption_01_Hard)))
  (Variables|System|Spawn|SetDifficultyTypeOption_02 (Utilities|Select :Index (LocalVariables|GetL_Difficulty) :NewEnumerator0 (Variables|Settings|Difficulty|Easy|GetDifficultySpawnOption_02_Easy) :NewEnumerator1 (Variables|Settings|Difficulty|Medium|GetDifficultySpawnOption_02_Medium) :NewEnumerator2 (Variables|Settings|Difficulty|Hard|GetDifficultySpawnOption_02_Hard)))
  ;[1 1 1] Set time changes by cubes and  transmit it ti BP_Player
  (Variables|System|TimeChangesByCubes|SetTimeChangeByGoodCube (Utilities|Select :Index (LocalVariables|GetL_Difficulty) :NewEnumerator0 (Variables|Settings|Difficulty|Easy|TimeChangesByCubes|GetTimeChangeByGoodCubeEasy) :NewEnumerator1 (Variables|Settings|Difficulty|Medium|TimeChangesByCubes|GetTimeChangeByGoodCubeMedium) :NewEnumerator2 (Variables|Settings|Difficulty|Hard|TimeChangesByCubes|GetTimeChangeByGoodCubeHard)))
  (Variables|System|TimeChangesbyCubes|SetTimeChangeByBadCube (Utilities|Select :Index (LocalVariables|GetL_Difficulty) :NewEnumerator0 (Variables|Settings|Difficulty|Easy|TimeChangesbyCubes|GetTimeChangeByBadCubeEasy) :NewEnumerator1 (Variables|Settings|Difficulty|Medium|TimeChangesbyCubes|GetTimeChangeByBadCubeMedium) :NewEnumerator2 (Variables|Settings|Difficulty|Hard|TimeChangesbyCubes|GetTimeChangeByBadCubeHard)))
  (Variables|System|TimeChangesbyCubes|SetTimeChangeByScoreCube (Utilities|Select :Index (LocalVariables|GetL_Difficulty) :NewEnumerator0 (Variables|Settings|Difficulty|Easy|TimeChangesbyCubes|GetTimeChangeByScoreCubeEasy) :NewEnumerator1 (Variables|Settings|Difficulty|Medium|TimeChangesbyCubes|GetTimeChangeByScoreCubeMedium) :NewEnumerator2 (Variables|Settings|Difficulty|Hard|TimeChangesbyCubes|GetTimeChangeByScoreCubeHard)))
  (Variables|System|TimeChangesbyCubes|SetTimeChangeByTimeCube (Utilities|Select :Index (LocalVariables|GetL_Difficulty) :NewEnumerator0 (Variables|Settings|Difficulty|Easy|TimeChangesbyCubes|GetTimeChangeByTimeCubeEasy) :NewEnumerator1 (Variables|Settings|Difficulty|Medium|TimeChangesbyCubes|GetTimeChangeByTimeCubeMedium) :NewEnumerator2 (Variables|Settings|Difficulty|Hard|TimeChangesbyCubes|GetTimeChangeByTimeCubeHard)))
  (Variables|System|TimeChangesbyCubes|SetTimeChangeByBonusCube (Utilities|Select :Index (LocalVariables|GetL_Difficulty) :NewEnumerator0 (Variables|Settings|Difficulty|Easy|TimeChangesbyCubes|GetTimeChangeByBonusCubeEasy) :NewEnumerator1 (Variables|Settings|Difficulty|Medium|TimeChangesbyCubes|GetTimeChangeByBonusCubeMedium) :NewEnumerator2 (Variables|Settings|Difficulty|Hard|TimeChangesbyCubes|GetTimeChangeByBonusCubeHard)))
  (Variables|System|TimeChangesbyCubes|SetTimeChangeBySpeedCube (Utilities|Select :Index (LocalVariables|GetL_Difficulty) :NewEnumerator0 (Variables|Settings|Difficulty|Easy|TimeChangesbyCubes|GetTimeChangeBySpeedCubeEasy) :NewEnumerator1 (Variables|Settings|Difficulty|Medium|TimeChangesbyCubes|GetTimeChangeBySpeedCubeMedium) :NewEnumerator2 (Variables|Settings|Difficulty|Hard|TimeChangesbyCubes|GetTimeChangeBySpeedCubeHard)))
  (Setters|SetTimeChangesbyCubeValues)
  ;[1 1 1] Set score changes by cubes and  transmit it ti BP_Player
  (Variables|System|ScoreChangeByCubes|SetScoreChangeByGoodCube (Utilities|Select :Index (LocalVariables|GetL_Difficulty) :NewEnumerator0 (Variables|Settings|Difficulty|Easy|ScoreChangesByCubes|GetScoreChangeByGoodCubeEasy) :NewEnumerator1 (Variables|Settings|Difficulty|Medium|ScoreChangesbyCubes|GetScoreChangeByGoodCubeMedium) :NewEnumerator2 (Variables|Settings|Difficulty|Hard|ScoreChangesByCubes|GetScoreChangeByGoodCubeHard)))
  (Variables|System|ScoreChangebyCubes|SetScoreChangeByBadCube (Utilities|Select :Index (LocalVariables|GetL_Difficulty) :NewEnumerator0 (Variables|Settings|Difficulty|Easy|ScoreChangesbyCubes|GetScoreChangeByBadCubeEasy) :NewEnumerator1 (Variables|Settings|Difficulty|Medium|ScoreChangesbyCubes|GetScoreChangeByBadCubeMedium) :NewEnumerator2 (Variables|Settings|Difficulty|Hard|ScoreChangesbyCubes|GetScoreChangeByBadCubeHard)))
  (Variables|System|ScoreChangebyCubes|SetScoreChangeByScoreCube (Utilities|Select :Index (LocalVariables|GetL_Difficulty) :NewEnumerator0 (Variables|Settings|Difficulty|Easy|ScoreChangesbyCubes|GetScoreChangeByScoreCubeEasy) :NewEnumerator1 (Variables|Settings|Difficulty|Medium|ScoreChangesByCubes|GetScoreChangeByScoreCubeMedium) :NewEnumerator2 (Variables|Settings|Difficulty|Hard|ScoreChangesbyCubes|GetScoreChangeByScoreCubeHard)))
  (Variables|System|ScoreChangebyCubes|SetScoreChangeByTimeCube (Utilities|Select :Index (LocalVariables|GetL_Difficulty) :NewEnumerator0 (Variables|Settings|Difficulty|Easy|ScoreChangesbyCubes|GetScoreChangeByTimeCubeEasy) :NewEnumerator1 (Variables|Settings|Difficulty|Medium|ScoreChangesByCubes|GetScoreChangeByTimeCubeMedium) :NewEnumerator2 (Variables|Settings|Difficulty|Hard|ScoreChangesbyCubes|GetScoreChangeByTimeCubeHard)))
  (Variables|System|ScoreChangebyCubes|SetScoreChangeByBonusCube (Utilities|Select :Index (LocalVariables|GetL_Difficulty) :NewEnumerator0 (Variables|Settings|Difficulty|Easy|ScoreChangesbyCubes|GetScoreChangeByBonusCubeEasy) :NewEnumerator1 (Variables|Settings|Difficulty|Medium|ScoreChangesByCubes|GetScoreChangeByBonusCubeMedium) :NewEnumerator2 (Variables|Settings|Difficulty|Hard|ScoreChangesbyCubes|GetScoreChangeByBonusCubeHard)))
  (Variables|System|ScoreChangebyCubes|SetScoreChangeBySpeedCube (Utilities|Select :Index (LocalVariables|GetL_Difficulty) :NewEnumerator0 (Variables|Settings|Difficulty|Easy|ScoreChangesbyCubes|GetScoreChangeBySpeedCubeEasy) :NewEnumerator1 (Variables|Settings|Difficulty|Medium|ScoreChangesByCubes|GetScoreChangeBySpeedCubeMedium) :NewEnumerator2 (Variables|Settings|Difficulty|Hard|ScoreChangesbyCubes|GetScoreChangeBySpeedCubeHard)))
  (Setters|SetScoreChangesbyCubeValues)
  ;[1 1 1] Set MaxMultiplyCount
  (Variables|System|SetMaxMultiplyCount (Utilities|Array|Length (Variables|Settings|GetMultiplyCubeSpawnPoints)))
  ;[1 1 1] Set number of spawn points
  (Variables|System|Spawn|SetSpawnPointsAmount (- (Utilities|Array|Length (Variables|Settings|GetCubeSpawnPonts)) 1))
  ;[1 1 1] Set ScoreToSpeedUp
  (Default|SetScoretoSpeedUp (Variables|System|GetBP_Player) (Utilities|Select :Index (LocalVariables|GetL_Difficulty) :NewEnumerator0 (Variables|Settings|Difficulty|Easy|GetScoreToSpeedUpEasy) :NewEnumerator1 (Variables|Settings|Difficulty|Medium|GetScoreToSpeedUpMedium) :NewEnumerator2 (Variables|Settings|Difficulty|Hard|GetScoreToSpeedUpHard)))
  (return))

(fn SpawnUIBonusCube
  (bind _output_get (LocalVariables|SetL_CurrentBonus (Default|GetCurrentBonus (Variables|/Game/Gameplay/Player/BP_Player.BP_Player_C|GetBPC_Bonus (Variables|System|GetBP_Player)))))
  (if (Utilities|Enum|Equal(Enum) _output_get "NewEnumerator3")
    (bind _spawnedui_bonuscube (Variables|System|Spawn|GetSpawnedUI_BonusCube)
      (:then
        (Default|Destructor _spawnedui_bonuscube)
        (Variables|System|Spawn|SetSpawnedUI_BonusCube 0)
        (return))
      (:else))
    (else
      (bind _spawnedui_bonuscube_2 (Variables|System|Spawn|GetSpawnedUI_BonusCube)
        (:then
          (Actor|DestroyActor _spawnedui_bonuscube_2))
        (:else
          _))
      (bind _returnvalue (Game|SpawnActorfromClass "/Game/Gameplay/Cubes/BP_UI_BonusCube.BP_UI_BonusCube_C" (Transformation|GetActorTransform (Variables|Settings|GetCurrentBonusSpawnPoint)) "Undefined" 0 (LocalVariables|GetL_CurrentBonus) 0))
      (Variables|System|Spawn|SetSpawnedUI_BonusCube _returnvalue)
      (return))))

(fn GetSpawnedUIMultiplyCubes
  (return (Variables|System|Spawn|GetSpawnedUI_MultiplyCubes)))

(fn GetSpawnedUIBonusCube
  (return (Variables|System|Spawn|GetSpawnedUI_BonusCube)))