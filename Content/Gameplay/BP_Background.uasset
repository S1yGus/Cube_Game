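; BP_Background is a music-visualizer backdrop that spawns a grid of BP_BackgroundCube actors and plays a sound on BeginPlay.
; It binds to audio playback percent and maps each sound wave to Constant-Q Synesthesia data, with the frequency variant chosen by the game instance.
; Synesthesia holds logic to drive cube height and scale, plus UI bonus cube height, from band values, but that logic is unreachable as wired.
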(event Custom|SpawnBackgroundCubes
  ;[1 1 1] Spawn matrix of cubes on background
  (for _index (range 0 (Variables|Settings|Background|GetRows))
    (for _index_2 (range 0 (Variables|Settings|Background|GetCols))
      (bind _returnvalue (Game|SpawnActorfromClass "/Game/Gameplay/Cubes/BackgroundCubes/BP_BackgroundCube.BP_BackgroundCube_C" (Math|Transform|MakeTransform (Math|Vector|MakeVector (+ (Variables|Settings|Background|GetColsOffset) (* _index_2 (Variables|Settings|Background|GetDistanceBetweenCubes))) (+ (Variables|Settings|Background|GetRowsOffset) (* _index (Variables|Settings|Background|GetDistanceBetweenCubes))) (Variables|Settings|Background|GetSpawnCubesLocationZ)) "0, 0, 0" "1.000000,1.000000,1.000000") "Undefined" 0 0))
      (Utilities|Array|Add (Variables|System|GetCubes) _returnvalue))))

(event EventBeginPlay
  (CallFunction|SpawnBackgroundCubes)
  (System|Constructor)
  (EventDispatchers|BindEventtoOnAudioPlaybackPercent (Variables|Default|GetAudio) (EventDispatchers|CreateEvent :!event Synesthesia))
  (Audio|Components|Audio|Play (Variables|Default|GetAudio) 0.0))

(fn ConstructionScript)

(fn Synesthesia
  (params (PlayingSoundWave :type Sound%20Wave%20Object%20Reference) (PlaybackPercent :type Float%20%28single-precision%29))
  ;[1 1 1] If there is synesthesia asset for current wave
  (if (not (.ReturnValue (Utilities|Map|Find (Variables|Settings|GetSynesthesiaMap) PlayingSoundWave)))
    (return)))

(fn Constructor
  (Audio|Components|Audio|SetSound (Variables|Default|GetAudio) (Variables|Settings|GetSound))
  (Variables|System|SetBP_GameInstance (.AsBP%20Game%20Instance (Utilities|Casting|CastToBP_GameInstance (Game|GetGameInstance)))))

(fn SelectSynesthesia
  (params (S_Synesthesia :type S%20Synesthesia%20Structure))
  (return (Utilities|Select :Index (System|GetSynesthesiaFrequency) :NewEnumerator0 (.highfrequency S_Synesthesia) :NewEnumerator1 (.mediumfrequency S_Synesthesia) :NewEnumerator2 (.lowfrequency S_Synesthesia))))

(fn GetSynesthesiaFrequency
  (return (Default|GetSynesthesiaFrequency (Variables|System|GetBP_GameInstance))))