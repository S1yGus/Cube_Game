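; BP_Cube_Base is a base cube actor that animates its scale when it appears and before it is destroyed.
; On BeginPlay it stores the current skin struct from BP_GameInstance, then a looping timer drives ChangeScale along an appearance curve until it nears MaxScale.
; Destructor runs the same curve-sampled scaling with a disappearance curve and destroys the actor once the mesh nearly reaches minimum size.
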(event Custom|Constructor
  (Variables|Default|SetCurrentSkin (Default|GetCurrentSkinStuct (System|GetGameInstance)))
  ;[1 1 1] Set begin play change scale timer
  (bind _returnvalue (Utilities|Time|SetTimerbyEvent (delegate Custom|ConstructorScale) (Variables|System|Scale|GetTimerRate) true))
  (Variables|System|Scale|SetConstructorScaleTimer _returnvalue))

(event Custom|Destructor
  (Utilities|Time|SetTimerbyEvent (delegate Custom|DestructorScale) (Variables|System|Scale|GetTimerRate) true))

(event Custom|ConstructorScale
  ;[1 1 1] Set begin play change scale timer
  (bind _changescalecompleted (System|ChangeScale (Variables|System|Scale|GetCurve_AppearanceScale) (Variables|System|Scale|GetMaxScale)))
  (if _changescalecompleted
    (Utilities|Time|ClearandInvalidateTimerbyHandle (Variables|System|Scale|GetConstructorScaleTimer))
    (Variables|System|Scale|SetTime 0.0)))

(event Custom|DestructorScale
  (bind _changescalecompleted (System|ChangeScale (Variables|System|Scale|GetCurve_DisappearanceScale) 0.01))
  (if _changescalecompleted
    (Actor|DestroyActor)))

(event EventBeginPlay
  (CallFunction|Constructor))

(fn ConstructionScript)

(fn ChangeScale
  (params (Curve :type Curve%20Float%20Object%20Reference) (TargetScale :type Float%20%28single-precision%29))
  (Variables|System|Scale|SetTime (+ (Variables|System|Scale|GetTime) (Variables|System|Scale|GetTimerRate)))
  (LocalVariables|SetL_CurveValue (Math|Curves|GetFloatValue Curve (Variables|System|Scale|GetTime)))
  (Transformation|SetWorldScale3D (Variables|Default|GetCubeStaticMesh) (Math|Vector|MakeVector (LocalVariables|GetL_CurveValue) (LocalVariables|GetL_CurveValue) (LocalVariables|GetL_CurveValue)))
  ;[1 1 1] If CurveValue == MaxScale stop timer
  (if (Math|Float|NearlyEqual(Float) (LocalVariables|GetL_CurveValue) TargetScale 0.01)
    (return true)
    (else
      (return false))))

(fn GetGameInstance
  (return (.AsBP%20Game%20Instance (Utilities|Casting|CastToBP_GameInstance (Game|GetGameInstance)))))