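; BP_UI_BonusCube is a cube Blueprint that, by its name, serves as the UI version of the bonus cube.
; Its Constructor event runs the parent logic, then calls SetSkin to apply a material to CubeStaticMesh.
; SetSkin picks that material from CurrentSkin by BonusType, covering missile, shield and bomb bonuses.
; BeginPlay and the construction script only call their parent versions.
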(event Custom|SetSkin
  (bind _currentskin (Variables|Default|GetCurrentSkin))
  (bind (_player _goodcube _badcube _scorecube _timecube _bonuscube _speedcube _bonuscubemissile _bonuscubeshield _bonuscubebomb) (Utilities|Struct|BreakS_Skin _currentskin))
  (Rendering|Material|SetMaterial (Variables|Default|GetCubeStaticMesh) 0 (Utilities|Select :Index (Variables|System|GetBonusType) :NewEnumerator3 0 :NewEnumerator0 _bonuscubemissile :NewEnumerator1 _bonuscubeshield :NewEnumerator2 _bonuscubebomb)))

(event EventBeginPlay
  (|CallParentFunction))

(event EventConstructor
  (|CallParentFunction)
  (CallFunction|SetSkin))

(fn ConstructionScript
  (|CallParentFunction))