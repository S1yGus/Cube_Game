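; BP_UIMultiplyCube is a cube Blueprint, apparently a UI variant of a gameplay cube, whose look reflects its cube type.
; After the parent BeginPlay, SetSkin selects a material from the CubeType enum, mostly neon instances plus a power-up one, and applies it to the static mesh's first slot.
; GetCubeType exposes the type, and the construction script only calls the parent.
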(event Custom|SetSkin
  (Rendering|Material|SetMaterial (Variables|Default|GetCubeStaticMesh) 0 (Utilities|Select :Index (Variables|System|GetCubeType) :NewEnumerator6 0 :NewEnumerator0 "/Game/Materials/Cubes/MI_GoodCubeNeon.MI_GoodCubeNeon" :NewEnumerator1 "/Game/Materials/Cubes/MI_BadCubeNeon.MI_BadCubeNeon" :NewEnumerator2 "/Game/Materials/Cubes/MI_ScoreCubeNeon.MI_ScoreCubeNeon" :NewEnumerator3 "/Game/Materials/Cubes/MI_TimeCubeNeon.MI_TimeCubeNeon" :NewEnumerator4 "/Game/Materials/Cubes/MI_BonusCubeNeon.MI_BonusCubeNeon" :NewEnumerator5 "/Game/Materials/Cubes/MI_SpeedCubeNeon.MI_SpeedCubeNeon" :NewEnumerator7 "/Game/Materials/PowerUp/MI_PowerUp.MI_PowerUp")))

(event EventBeginPlay
  (|CallParentFunction)
  (CallFunction|SetSkin))

(fn ConstructionScript
  (|CallParentFunction))

(fn GetCubeType
  (return (Variables|System|GetCubeType)))