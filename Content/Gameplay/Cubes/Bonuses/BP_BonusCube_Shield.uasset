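; Shield bonus cube that makes the player temporarily immune to catching cubes by disabling the player's collision box.
; On BeginPlay it turns that collision off and starts a looping timer that moves the shield actor onto the player cube's location.
; After the action time elapses, it restores query-only collision and calls its Destructor.
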(event Custom|Shield
  ;[1 1 1] Set ShieldBonus location to follow BP_Player
  (Transformation|SetActorLocation (Transformation|GetWorldLocation (Variables|/Game/Gameplay/Player/BP_Player.BP_Player_C|GetPlayerCube (Variables|System|GetBP_Player))) false false))

(event EventBeginPlay
  (|CallParentFunction)
  (Variables|System|SetBP_Player (.AsBP%20Player (Utilities|Casting|CastToBP_Player (Game|Player|GetPlayerPawn 0))))
  ;[1 0.151 0.151] To avoid issue with catching cubes
  (System|SetPlayerCollision "NoCollision")
  ;[1 1 1] Set ShieldBonus location to follow BP_Player
  (Utilities|Time|SetTimerbyEvent (delegate Custom|Shield) (Variables|Default|GetTimerRate) true)
  ;[1 1 1] Time of action
  (Utilities|FlowControl|Delay (Variables|System|GetTimeOfAction))
  ;[0.6615 0.08268 0.08268] Return BP_Player collision
  (System|SetPlayerCollision "QueryOnly")
  (CallFunction|Destructor))

(fn ConstructionScript
  (|CallParentFunction))

(fn SetPlayerCollision
  (params (Set%20collision :type ECollisionEnabled%20Enum :default "NoCollision"))
  (Collision|SetCollisionEnabled (Variables|/Game/Gameplay/Player/BP_Player.BP_Player_C|GetPlayerCollisionBox (Variables|System|GetBP_Player)) Set%20collision)
  (return))