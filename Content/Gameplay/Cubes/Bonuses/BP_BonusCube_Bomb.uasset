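; BP_BonusCube_Bomb is a timed bomb bonus cube that follows the player.
; On BeginPlay it runs the parent logic, caches the BP_Player pawn and starts a looping timer that snaps the actor to the PlayerCube's world location every TimerRate seconds.
; After a TimeOfAction delay it calls Destructor to end the bonus.
; No explosion or damage logic is defined in this Blueprint itself.
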(event Custom|Bomb
  ;[1 1 1] Set BombBonus location to follow BP_Player
  (Transformation|SetActorLocation (Transformation|GetWorldLocation (Variables|/Game/Gameplay/Player/BP_Player.BP_Player_C|GetPlayerCube (Variables|Default|GetBP_Player))) false false))

(event EventBeginPlay
  (|CallParentFunction)
  (Variables|Default|SetBP_Player (.AsBP%20Player (Utilities|Casting|CastToBP_Player (Game|Player|GetPlayerPawn 0))))
  ;[1 1 1] Set BombBonus location to follow BP_Player
  (Utilities|Time|SetTimerbyEvent (delegate Custom|Bomb) (Variables|Default|GetTimerRate) true)
  ;[1 1 1] Time of action
  (Utilities|FlowControl|Delay (Variables|Default|GetTimeOfAction))
  (CallFunction|Destructor))

(fn ConstructionScript
  (|CallParentFunction))