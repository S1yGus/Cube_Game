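; BP_UI_MultipyCube is a cube Blueprint that displays the current skin's material for its cube type.
; On BeginPlay it runs the parent logic, then SetSkin selects the CurrentSkin material matching CubeType and applies it to the first material slot of CubeStaticMesh.
; GetCubeType exposes the type, and the construction script only calls the parent.
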(event Custom|SetSkin
  (bind _currentskin (Variables|Default|GetCurrentSkin))
  (bind (_player _goodcube _badcube _scorecube _timecube _bonuscube _speedcube _bonuscubemissile _bonuscubeshield _bonuscubebomb _powerup) (Utilities|Struct|BreakS_Skin _currentskin))
  ;[1 1 1] Set skin
  (Rendering|Material|SetMaterial (Variables|Default|GetCubeStaticMesh) 0 (Utilities|Select :Index (Variables|System|GetCubeType) :NewEnumerator0 _goodcube :NewEnumerator1 _badcube :NewEnumerator2 _scorecube :NewEnumerator3 _timecube :NewEnumerator4 _bonuscube :NewEnumerator5 _speedcube :NewEnumerator7 _powerup :NewEnumerator6 0)))

(event EventBeginPlay
  (|CallParentFunction)
  (CallFunction|SetSkin))

(fn ConstructionScript
  (|CallParentFunction))

(fn GetCubeType
  (return (Variables|System|GetCubeType)))