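; BP_UIBonusCube is a cube Blueprint that shows a bonus type through its material, apparently as a display piece for the UI.
; Its Constructor event runs the parent logic, then calls SetSkin to pick the missile, shield or bomb material from BonusType and apply it to CubeStaticMesh.
; The None type has no material assigned, and BeginPlay and the construction script only call their parents.
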(event Custom|SetSkin
  (Rendering|Material|SetMaterial (Variables|Default|GetCubeStaticMesh) 0 (Utilities|Select :Index (Variables|System|GetBonusType) :NewEnumerator3 0 :NewEnumerator0 "/Game/Materials/Bonuses/MI_MissileBonus.MI_MissileBonus" :NewEnumerator1 "/Game/Materials/Bonuses/MI_ShieldBonus.MI_ShieldBonus" :NewEnumerator2 "/Game/Materials/Bonuses/MI_BombBonus.MI_BombBonus")))

(event EventBeginPlay
  (|CallParentFunction))

(event EventConstructor
  (|CallParentFunction)
  (CallFunction|SetSkin))

(fn ConstructionScript
  (|CallParentFunction))