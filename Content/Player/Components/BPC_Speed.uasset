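; BPC_Speed is a player component that holds a Speed count and exposes a getter for it.
; IncreaseSpeed adds one with no upper limit, while DecreaseSpeed subtracts one and clamps the result at a minimum of one.
; Both functions then fire the EDSpeedChanged event dispatcher, even when a decrease leaves the value at the floor.
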(fn GetSpeedCount
  (return (Variables|System|GetSpeed)))

(fn IncreaseSpeed
  (Math|Integer|IncrementInt (Variables|System|GetSpeed)
    (:%20%20
      (Default|CallEDSpeedChanged)
      (return))))

(fn DecreaseSpeed
  (Variables|System|SetSpeed (Math|Integer|Max(Integer) (- (Variables|System|GetSpeed) 1) 1))
  (Default|CallEDSpeedChanged)
  (return))