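; Score component that tracks the player's score and triggers speed increases at point thresholds.
; ChangeScore adds to both the score, clamped at zero, and a speed-up counter, then fires the ScoreChanged dispatcher.
; When the counter reaches the GetScoreToSpeedUp threshold, it resets to the score's remainder and the owner is cast to BP_Player for the speed increase.
; GetScoreToSpeedUp casts the game mode to BP_GameMode, though both branches show zero.
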(fn ChangeScore
  (params (AddScore :type Integer))
  ;[1 1 1] Accumulate speed up score
  (Variables|System|SetSpeedUpScore (+ AddScore (Variables|System|GetSpeedUpScore)))
  ;[1 1 1] Accumulate score
  (Variables|System|SetScore (Math|Integer|Max(Integer) (+ AddScore (Variables|System|GetScore))))
  (Default|CallEDScoreChanged)
  ;[1 1 1] If SpeedUpScore > ScoreToSpeedUp - 1, then increase speed and set new SpeedUpScore
  (if (>= (Variables|System|GetSpeedUpScore) (CallFunction|GetScoretoSpeedUp))
    (Variables|System|SetSpeedUpScore (Math|Integer|%(Integer) (Variables|System|GetScore) (CallFunction|GetScoretoSpeedUp)))
    (Utilities|Casting|CastToBP_Player (Components|GetOwner)
      (:then
        (return))
      (:CastFailed
        (return)))
    (else
      (return))))

(fn GetScoretoSpeedUp
  (Utilities|Casting|CastToBP_GameMode (Game|GetGameMode)
    (:then
      (return 0))
    (:CastFailed
      (return 0))))