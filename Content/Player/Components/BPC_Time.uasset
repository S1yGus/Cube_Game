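; BPC_Time is a player component that holds a countdown clock in seconds and starts a looping one-second timer on BeginPlay.
; Countdown decrements Seconds and fires the time-changed dispatcher, also signalling low time whenever Seconds is at or below LowTime.
; At zero it stops decrementing and only casts to BP_GameMode, with no further action shown.
; ChangeTime adjusts the clock, clamped at zero, and broadcasts the change; GetTime returns the remaining seconds.
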(event EventBeginPlay
  (Utilities|Time|SetTimerbyEvent (EventDispatchers|CreateEvent :!event Countdown) 1.0 true))

(fn ChangeTime
  (params (AddSeconds :type Integer))
  (Variables|System|SetSeconds (Math|Integer|Max(Integer) (+ AddSeconds (Variables|System|GetSeconds))))
  (Default|CallEDTimeChanged)
  (return))

(fn GetTime
  (return (Variables|System|GetSeconds)))

(fn Countdown
  (if (<= (Variables|System|GetSeconds) (Variables|System|GetLowTime))
    (Default|CallEDLowTime))
  (if (== (Variables|System|GetSeconds) 0)
    (Utilities|Casting|CastToBP_GameMode (Game|GetGameMode)
      (:CastFailed
        (return)))
    (else
      (Math|Integer|DecrementInt (Variables|System|GetSeconds)
        (:%20%20
          (Default|CallEDTimeChanged)
          (return))))))