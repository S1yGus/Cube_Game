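; Runs the cube game: applies Game Instance difficulty to spawning and pushes per-cube time and score values to BP_Player.
; A looping timer at spacing divided by player speed spawns weighted random cubes, recursing by chance onto unique points up to a depth cap.
; Player multiplier changes spawn or clear BP_MultiplyCube indicators, with DoOnce limiting the spawn at maximum.
; A second timer drives a curve-based emissive pulse through a material parameter collection.
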(event Custom|MultiplyChange
  (bind _bp_player (Variables|Settings|GetBP_Player))
  (bind (_multiplycount _cubetype) (Default|GetMultiplyInfo _bp_player))
  ;[1 1 1] Multiply change
  (bind _output_get (Variables|System|SetCurrentMultiplyCount _multiplycount))
  (if (== _output_get 0)
    (bind _outactors (Actor|GetAllActorsOfClass "/Game/Base/Blueprints/Cubes/BP_MultiplyCube.BP_MultiplyCube_C"))
    (for _array_element _outactors
      (Default|Destructor (.AsBP%20Multiply%20Cube (Utilities|Casting|CastToBP_MultiplyCube _array_element)))
      (CallFunction|MultiplyReset))
    (else
      ;;[1 1 1] If CurrentMultiplyCount == MaxMultiplyCount spawn cube only one times
      (if (== (Variables|System|GetCurrentMultiplyCount) (Variables|System|GetMaxMultiplyCount))
        (Utilities|FlowControl|DoOnce false
          (:Completed
            _)))
      (Game|SpawnActorfromClass "/Game/Base/Blueprints/Cubes/BP_MultiplyCube.BP_MultiplyCube_C" (Transformation|GetActorTransform (Utilities|Array|Get(acopy) (Variables|Settings|GetMultiplyCubeSpawnPoints) (- (Variables|System|GetCurrentMultiplyCount) 1))) "Undefined" 0 (Utilities|Select :Index _cubetype :NewEnumerator0 "/Game/Materials/Cubes/MI_GoodCube.MI_GoodCube" :NewEnumerator1 "/Game/Materials/Cubes/MI_BadCube.MI_BadCube" :NewEnumerator2 "/Game/Materials/Cubes/MI_ScoreCub.MI_ScoreCub" :NewEnumerator3 "/Game/Materials/Cubes/MI_TimeCube.MI_TimeCube" :NewEnumerator4 "/Game/Materials/Cubes/MI_BonusCube.MI_BonusCube" :NewEnumerator5 "/Game/Materials/Cubes/MI_SpeedCube.MI_SpeedCube") 0))))

(event Custom|SetSpawnTimer
  ;[1 1 1] Set cpawn cube timer
  (if (Utilities|Time|IsValidTimerHandle (Variables|System|Spawn|GetSpawnCubeTimer))
    (Utilities|Time|ClearandInvalidateTimerbyHandle (Variables|System|Spawn|GetSpawnCubeTimer)))
  (bind _returnvalue (Utilities|Time|SetTimerbyEvent (EventDispatchers|CreateEvent :!event SpawnCubes) (System|GetTimerRate) true))
  (Variables|System|Spawn|SetSpawnCubeTimer _returnvalue))

(event Custom|MultiplyReset
  ;[1 1 1] Multiply change
  ;;[1 1 1] If CurrentMultiplyCount == MaxMultiplyCount spawn cube only one times
  (Utilities|FlowControl|DoOnce false) ; enters at Reset
)

(event EventBeginPlay
  (System|Initialization)
  ;[1 1 1] Start spawn cube timer
  (EventDispatchers|BindEventtoEDChangeSpeed (Variables|/Game/Base/Blueprints/Player/BP_Player.BP_Player_C|GetBPC_TimeScoreSpeed (System|GetBPPlayer)) (EventDispatchers|CreateEvent :!event Custom|SetSpawnTimer))
  (CallFunction|SetSpawnTimer)
  ;[1 1 1] Multiply change
  (EventDispatchers|BindEventtoEDMultiplyChange (Variables|Settings|GetBP_Player) (EventDispatchers|CreateEvent :!event Custom|MultiplyChange))
  ;[1 1 1] Set cube emmisive color pulse timer
  (Utilities|Time|SetTimerbyEvent (EventDispatchers|CreateEvent :!event CubeEmissivePulse) (Variables|Settings|CubeEmissivePulse|GetEmissivePulseTimeRate) true))

(fn ConstructionScript)

(fn GetBPPlayer
  (return (.AsBP%20Player (Utilities|Casting|CastToBP_Player (Game|Player|GetPlayerPawn 0)))))

(fn SpawnCubes
  ;[1 1 1] Current recursion count
  (Math|Integer|IncrementInt (Variables|System|Spawn|GetCurrentRecursionDepth)
    (:%20%20
      (if (<= (Variables|System|Spawn|GetCurrentRecursionDepth) (Variables|System|Spawn|GetMaxRecursionDepth))
        ;[1 1 1] Until get a unique spawn poin number
        (while (LocalVariables|GetL_NeedUniqueValue)
          ;[1 1 1] Get random spawn point number, if it already was used in this recursion cycle get another one
          (LocalVariables|SetL_CurrentRndomPointNumber (Math|Random|RandomIntegerinRange 0 (Variables|System|Spawn|GetSpawnPointsAmount)))
          (if (not (Utilities|Array|ContainsItem (Variables|System|Spawn|GetPreviousSpawnPointsNumbers) (LocalVariables|GetL_CurrentRndomPointNumber)))
            (LocalVariables|SetL_NeedUniqueValue false)))
        ;[1 1 1] Add new unique spawn point number to previous spawn points numbers
        (Utilities|Array|Add (Variables|System|Spawn|GetPreviousSpawnPointsNumbers) (LocalVariables|GetL_CurrentRndomPointNumber))
        ;[1 1 1] Spawn random cube
        (Game|SpawnActorfromClass (System|GetRandomCube) (Transformation|GetActorTransform (Utilities|Array|Get(acopy) (Variables|Settings|GetCubeSpawnPonts) (LocalVariables|GetL_CurrentRndomPointNumber))) "Undefined" 0 0)
        ;[1 1 1] Chance to trigger recursion
        (if (Math|Random|RandomBoolwithWeight (Variables|System|Spawn|GetChanceToTriggerRecursion))
          (System|SpawnCubes)
          (return)
          (else
            ;[1 1 1] End recursion
            (Variables|System|Spawn|SetCurrentRecursionDepth 0)
            (Utilities|Array|Clear (Variables|System|Spawn|GetPreviousSpawnPointsNumbers))
            (return)))
        (else
          ;[1 1 1] End recursion
          (Variables|System|Spawn|SetCurrentRecursionDepth 0)
          (Utilities|Array|Clear (Variables|System|Spawn|GetPreviousSpawnPointsNumbers))
          (return))))))

(fn GetTimerRate
  (return (/ (Variables|System|GetDistanceBetweenCubes) (Default|GetSpeed (Variables|/Game/Base/Blueprints/Player/BP_Player.BP_Player_C|GetBPC_TimeScoreSpeed (.AsBP%20Player (Utilities|Casting|CastToBP_Player (Game|Player|GetPlayerPawn 0))))))))

(fn CubeEmissivePulse
  (Rendering|Material|SetScalarParameterValue "/Game/Materials/MPC_Cubes.MPC_Cubes" "EmissivePulse" (Math|Curves|GetFloatValue (Variables|Settings|CubeEmissivePulse|GetCurveEmissivePower) (Variables|System|CubeEmissivePulse|GetCurveTime)) :!class /Script/Engine.KismetMaterialLibrary)
  (Variables|System|CubeEmissivePulse|SetCurveTime (+ (Variables|System|CubeEmissivePulse|GetCurveTime) (Variables|Settings|CubeEmissivePulse|GetEmissivePulseTimeRate)))
  (if (> (Variables|System|CubeEmissivePulse|GetCurveTime) 3.0)
    (Variables|System|CubeEmissivePulse|SetCurveTime 0.0))
  (return))

(fn SetTimeChangesbyCubeValues
  (Default|SetTimeChangebyCubesValues (Variables|Settings|GetBP_Player) (Variables|System|TimeChangesByCubes|GetTimeChangeByGoodCube) (Variables|System|TimeChangesbyCubes|GetTimeChangeByBadCube) (Variables|System|TimeChangesbyCubes|GetTimeChangeByScoreCube) (Variables|System|TimeChangesbyCubes|GetTimeChangeByTimeCube) (Variables|System|TimeChangesbyCubes|GetTimeChangeByBonusCube) (Variables|System|TimeChangesbyCubes|GetTimeChangeBySpeedCube))
  (return))

(fn SetScoreChangesbyCubeValues
  (Default|SetScoreChanbebyCubesValues (Variables|Settings|GetBP_Player) (Variables|Settings|ScoreChangeByCubes|GetScoreChangeByGoodCube) (Variables|Settings|ScoreChangebyCubes|GetScoreChangeByBadCube) (Variables|Settings|ScoreChangebyCubes|GetScoreChangeByScoreCube) (Variables|Settings|ScoreChangebyCubes|GetScoreChangeByTimeCube) (Variables|Settings|ScoreChangebyCubes|GetScoreChangeByBonusCube) (Variables|Settings|ScoreChangebyCubes|GetScoreChangeBySpeedCube))
  (return))

(fn GetRandomCube
  (bind _spawngoodcube (Variables|System|Spawn|GetSpawnGoodCube))
  (bind _spawnbadcube (Variables|System|Spawn|GetSpawnBadCube))
  (return (Utilities|Select :Index (Math|Random|RandomIntegerinRange 0 15) :Option%200 _spawngoodcube :Option%201 _spawngoodcube :Option%202 _spawngoodcube :Option%203 _spawngoodcube :Option%204 _spawngoodcube :Option%205 _spawnbadcube :Option%206 _spawnbadcube :Option%207 _spawnbadcube :Option%208 _spawnbadcube :Option%209 _spawnbadcube :Option%2010 (Variables|System|Spawn|GetSpawnScoreCube) :Option%2011 (Variables|System|Spawn|GetSpawnTimeCube) :Option%2012 (select (Math|Random|RandomBool) (Variables|System|Spawn|GetDifficultySpawnOption_01) (Variables|System|Spawn|GetSpawnBonusCube)) :Option%2013 (select (Math|Random|RandomBool) (Variables|System|Spawn|GetDifficultySpawnOption_02) (Variables|System|Spawn|GetSpawnSpeedCube)) :Option%2014 (Variables|System|Spawn|GetDifficultySpawnOption_01) :Option%2015 (Variables|System|Spawn|GetDifficultySpawnOption_02))))

(fn Initialization
  (System|SetDifficultySettings)
  (Utilities|IsValid (Variables|Settings|GetBP_Player)
    (:Is%20Valid
      (Setters|SetTimeChangesbyCubeValues)
      (Setters|SetScoreChangesbyCubeValues)
      (return))))

(fn SetDifficultySettings
  ;[1 1 1] Get difficulty from game instace
  (LocalVariables|SetL_Difficulty (Default|GetDifficulty (.AsBP%20Game%20Instance (Utilities|Casting|CastToBP_GameInstance (Game|GetGameInstance)))))
  ;[1 1 1] Set distance between cubes
  (Variables|System|SetDistanceBetweenCubes (Utilities|Select :Index (LocalVariables|GetL_Difficulty) :NewEnumerator0 (Variables|Settings|Difficulty|Easy|GetDistanceBetweenCubesEasy) :NewEnumerator1 (Variables|Settings|Difficulty|Medium|GetDistanceBetweenCubesMedium) :NewEnumerator2 (Variables|Settings|Difficulty|Hard|GetDistanceBetweenCubesHard)))
  ;[1 1 1] Set max recursion depth
  (Variables|System|Spawn|SetMaxRecursionDepth (Utilities|Select :Index (LocalVariables|GetL_Difficulty) :NewEnumerator0 (Variables|Settings|Difficulty|Easy|GetMaxRecursionDepthEasy) :NewEnumerator1 (Variables|Settings|Difficulty|Medium|GetMaxRecursionDepthMedium) :NewEnumerator2 (Variables|Settings|Difficulty|Hard|GetMaxRecursionDepthHard)))
  ;[1 1 1] Set spawn options
  (Variables|System|Spawn|SetDifficultySpawnOption_01 (Utilities|Select :Index (LocalVariables|GetL_Difficulty) :NewEnumerator0 (Variables|Settings|Difficulty|Easy|GetDifficultySpawnOption_01Easy) :NewEnumerator1 (Variables|Settings|Difficulty|Medium|GetDifficultySpawnOption_01Medium) :NewEnumerator2 (Variables|Settings|Difficulty|Hard|GetDifficultySpawnOption_01Hard)))
  (Variables|System|Spawn|SetDifficultySpawnOption_02 (Utilities|Select :Index (LocalVariables|GetL_Difficulty) :NewEnumerator0 (Variables|Settings|Difficulty|Easy|GetDifficultySpawnOption_02Easy) :NewEnumerator1 (Variables|Settings|Difficulty|Medium|GetDifficultySpawnOption_02Medium) :NewEnumerator2 (Variables|Settings|Difficulty|Hard|GetDifficultySpawnOption_02Hard)))
  ;[1 1 1] Time changes by cubes
  (Variables|System|TimeChangesByCubes|SetTimeChangeByGoodCube (Utilities|Select :Index (LocalVariables|GetL_Difficulty) :NewEnumerator0 (Variables|Settings|Difficulty|Easy|TimeChangesByCubes|GetTimeChangeByGoodCubeEasy) :NewEnumerator1 (Variables|Settings|Difficulty|Medium|TimeChangesByCubes|GetTimeChangeByGoodCubeMedium) :NewEnumerator2 (Variables|Settings|Difficulty|Hard|TimeChangesByCubes|GetTimeChangeByGoodCubeHard)))
  (Variables|System|TimeChangesbyCubes|SetTimeChangeByBadCube (Utilities|Select :Index (LocalVariables|GetL_Difficulty) :NewEnumerator0 (Variables|Settings|Difficulty|Easy|TimeChangesbyCubes|GetTimeChangeByBadCubeEasy) :NewEnumerator1 (Variables|Settings|Difficulty|Medium|TimeChangesbyCubes|GetTimeChangeByBadCubeMedium) :NewEnumerator2 (Variables|Settings|Difficulty|Hard|TimeChangesbyCubes|GetTimeChangeByBadCubeHard)))
  (Variables|System|TimeChangesbyCubes|SetTimeChangeByScoreCube (Utilities|Select :Index (LocalVariables|GetL_Difficulty) :NewEnumerator0 (Variables|Settings|Difficulty|Easy|TimeChangesbyCubes|GetTimeChangeByScoreCubeEasy) :NewEnumerator1 (Variables|Settings|Difficulty|Medium|TimeChangesbyCubes|GetTimeChangeByScoreCubeMedium) :NewEnumerator2 (Variables|Settings|Difficulty|Hard|TimeChangesbyCubes|GetTimeChangeByScoreCubeHard)))
  (Variables|System|TimeChangesbyCubes|SetTimeChangeByTimeCube (Utilities|Select :Index (LocalVariables|GetL_Difficulty) :NewEnumerator0 (Variables|Settings|Difficulty|Easy|TimeChangesbyCubes|GetTimeChangeByTimeCubeEasy) :NewEnumerator1 (Variables|Settings|Difficulty|Medium|TimeChangesbyCubes|GetTimeChangeByTimeCubeMedium) :NewEnumerator2 (Variables|Settings|Difficulty|Hard|TimeChangesbyCubes|GetTimeChangeByTimeCubeHard)))
  (Variables|System|TimeChangesbyCubes|SetTimeChangeByBonusCube (Utilities|Select :Index (LocalVariables|GetL_Difficulty) :NewEnumerator0 (Variables|Settings|Difficulty|Easy|TimeChangesbyCubes|GetTimeChangeByBonusCubeEasy) :NewEnumerator1 (Variables|Settings|Difficulty|Medium|TimeChangesbyCubes|GetTimeChangeByBonusCubeMedium) :NewEnumerator2 (Variables|Settings|Difficulty|Hard|TimeChangesbyCubes|GetTimeChangeByBonusCubeHard)))
  (Variables|System|TimeChangesbyCubes|SetTimeChangeBySpeedCube (Utilities|Select :Index (LocalVariables|GetL_Difficulty) :NewEnumerator0 (Variables|Settings|Difficulty|Easy|TimeChangesbyCubes|GetTimeChangeBySpeedCubeEasy) :NewEnumerator1 (Variables|Settings|Difficulty|Medium|TimeChangesbyCubes|GetTimeChangeBySpeedCubeMedium) :NewEnumerator2 (Variables|Settings|Difficulty|Hard|TimeChangesbyCubes|GetTimeChangeBySpeedCubeHard)))
  ;[1 1 1] Score changes by cubes
  (Variables|Settings|ScoreChangeByCubes|SetScoreChangeByGoodCube (Utilities|Select :Index (LocalVariables|GetL_Difficulty) :NewEnumerator0 (Variables|Settings|Difficulty|Easy|ScoreChangesByCubes|GetScoreChangeByGoodCubeEasy) :NewEnumerator1 (Variables|Settings|Difficulty|Medium|ScoreChangesbyCubes|GetScoreChangeByGoodCubeMedium) :NewEnumerator2 (Variables|Settings|Difficulty|Hard|ScoreChangesByCubes|GetScoreChangeByGoodCubeHard)))
  (Variables|Settings|ScoreChangebyCubes|SetScoreChangeByBadCube (Utilities|Select :Index (LocalVariables|GetL_Difficulty) :NewEnumerator0 (Variables|Settings|Difficulty|Easy|ScoreChangesbyCubes|GetScoreChangeByBadCubeEasy) :NewEnumerator1 (Variables|Settings|Difficulty|Medium|ScoreChangesbyCubes|GetScoreChangeByBadCubeMedium) :NewEnumerator2 (Variables|Settings|Difficulty|Hard|ScoreChangesbyCubes|GetScoreChangeByBadCubeHard)))
  (Variables|Settings|ScoreChangebyCubes|SetScoreChangeByScoreCube (Utilities|Select :Index (LocalVariables|GetL_Difficulty) :NewEnumerator0 (Variables|Settings|Difficulty|Easy|ScoreChangesbyCubes|GetScoreChangeByScoreCubeEasy) :NewEnumerator1 (Variables|Settings|Difficulty|Medium|ScoreChangesByCubes|GetScoreChangeByScoreCubeMedium) :NewEnumerator2 (Variables|Settings|Difficulty|Hard|ScoreChangesbyCubes|GetScoreChangeByScoreCubeHard)))
  (Variables|Settings|ScoreChangebyCubes|SetScoreChangeByTimeCube (Utilities|Select :Index (LocalVariables|GetL_Difficulty) :NewEnumerator0 (Variables|Settings|Difficulty|Easy|ScoreChangesbyCubes|GetScoreChangeByTimeCubeEasy) :NewEnumerator1 (Variables|Settings|Difficulty|Medium|ScoreChangesByCubes|GetScoreChangeByTimeCubeMedium) :NewEnumerator2 (Variables|Settings|Difficulty|Hard|ScoreChangesbyCubes|GetScoreChangeByTimeCubeHard)))
  (Variables|Settings|ScoreChangebyCubes|SetScoreChangeByBonusCube (Utilities|Select :Index (LocalVariables|GetL_Difficulty) :NewEnumerator0 (Variables|Settings|Difficulty|Easy|ScoreChangesbyCubes|GetScoreChangeByBonusCubeEasy) :NewEnumerator1 (Variables|Settings|Difficulty|Medium|ScoreChangesByCubes|GetScoreChangeByBonusCubeMedium) :NewEnumerator2 (Variables|Settings|Difficulty|Hard|ScoreChangesbyCubes|GetScoreChangeByBonusCubeHard)))
  (Variables|Settings|ScoreChangebyCubes|SetScoreChangeBySpeedCube (Utilities|Select :Index (LocalVariables|GetL_Difficulty) :NewEnumerator0 (Variables|Settings|Difficulty|Easy|ScoreChangesbyCubes|GetScoreChangeBySpeedCubeEasy) :NewEnumerator1 (Variables|Settings|Difficulty|Medium|ScoreChangesByCubes|GetScoreChangeBySpeedCubeMedium) :NewEnumerator2 (Variables|Settings|Difficulty|Hard|ScoreChangesbyCubes|GetScoreChangeBySpeedCubeHard)))
  ;[1 1 1] Set MaxMultiplyCount
  (Variables|System|SetMaxMultiplyCount (Utilities|Array|Length (Variables|Settings|GetMultiplyCubeSpawnPoints)))
  ;[1 1 1] Set number of spawn points
  (Variables|System|Spawn|SetSpawnPointsAmount (- (Utilities|Array|Length (Variables|Settings|GetCubeSpawnPonts)) 1))
  (return))