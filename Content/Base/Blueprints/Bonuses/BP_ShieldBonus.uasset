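; Temporary shield bonus actor that protects the player and destroys cubes it touches.
; On BeginPlay it disables the player's collision box to avoid catching cubes and starts a looping timer.
; Each tick of that timer moves the shield mesh to the player's cube and scales the actor from a float curve.
; After five seconds it restores player collision, plays a finish sound and destroys itself.
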(event OnComponentBeginOverlap(ShieldCollisionBox)
  (params (OverlappedComponent :type Primitive%20Component%20Object%20Reference) (OtherActor :type Actor%20Object%20Reference) (OtherComp :type Primitive%20Component%20Object%20Reference) (OtherBodyIndex :type Integer) (bFromSweep :type Boolean) (SweepResult :type Hit%20Result%20Structure%20%28by%20ref%29))
  (bind _asbp_base_cube (Utilities|Casting|CastToBP_BaseCube OtherActor))
  (Actor|DestroyActor _asbp_base_cube))

(event Custom|Shield
  ;[1 1 1] Set ShieldBonus location to follow BP_Player
  (Transformation|SetWorldLocation (Variables|Default|GetShieldStaticMesh) (Transformation|GetWorldLocation (Variables|/Game/Base/Blueprints/Player/BP_Player.BP_Player_C|GetPlayerCube (CallFunction|GetBPPlayer))) false false)
  ;[1 1 1] Set ShieldBonus scale
  (Transformation|SetActorScale3D (Math|Vector|MakeVector (Math|Curves|GetFloatValue (Variables|System|GetShieldCurve) (Variables|System|GetInTime)) (Math|Curves|GetFloatValue (Variables|System|GetShieldCurve) (Variables|System|GetInTime)) (Math|Curves|GetFloatValue (Variables|System|GetShieldCurve) (Variables|System|GetInTime))))
  ;[1 1 1] Increase inTime
  (bind _output_get (Variables|System|SetInTime (+ (Variables|System|GetInTime) (Variables|System|GetTimerRate))))
  (if (>= _output_get 5.0)
    ;[1 1 1] Return BP_Player collision
    (CallFunction|SetBPPlayerCollision "QueryAndPhysics")
    (Audio|PlaySound2D (Variables|System|GetFinishSound) 1.0 1.0 0.0 0 0)
    (Actor|DestroyActor)))

(event EventBeginPlay
  (Audio|PlaySound2D (Variables|System|GetInitialSound) 1.0 1.0 0.0 0 0)
  ;[1 1 1] To avoid issue with catching cubes
  (CallFunction|SetBPPlayerCollision "NoCollision")
  (Utilities|Time|SetTimerbyEvent (delegate Custom|Shield) (Variables|System|GetTimerRate) true))

(fn ConstructionScript)

(fn GetBPPlayer
  (return (.AsBP%20Player (Utilities|Casting|CastToBP_Player (Game|Player|GetPlayerPawn 0)))))

(fn SetBPPlayerCollision
  (params (Set%20collision :type ECollisionEnabled%20Enum :default "NoCollision"))
  (Collision|SetCollisionEnabled (Variables|/Game/Base/Blueprints/Player/BP_Player.BP_Player_C|GetPlayerCollisionBox (CallFunction|GetBPPlayer)) Set%20collision)
  (return))