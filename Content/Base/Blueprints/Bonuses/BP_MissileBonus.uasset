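; BP_MissileBonus is a missile that destroys the cube it hits.
; On BeginPlay it plays a launch sound and sets its projectile movement velocity along local Z at MissileSpeed.
; When its collision box overlaps a BP_BaseCube, it destroys that cube, plays a hit sound and destroys itself, ignoring all other actors.
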(event OnComponentBeginOverlap(MissileCollisionBox)
  (params (OverlappedComponent :type Primitive%20Component%20Object%20Reference) (OtherActor :type Actor%20Object%20Reference) (OtherComp :type Primitive%20Component%20Object%20Reference) (OtherBodyIndex :type Integer) (bFromSweep :type Boolean) (SweepResult :type Hit%20Result%20Structure%20%28by%20ref%29))
  (bind _asbp_base_cube (Utilities|Casting|CastToBP_BaseCube OtherActor))
  (Actor|DestroyActor _asbp_base_cube)
  (Audio|PlaySound2D (Variables|System|GetHitSound) 1.0 1.0 0.0 0 0)
  (Actor|DestroyActor))

(event EventBeginPlay
  (Audio|PlaySound2D (Variables|System|GetInitialSound) 1.0 1.0 0.0 0 0)
  (System|Moving))

(fn ConstructionScript)

(fn Moving
  (Game|Components|ProjectileMovement|SetVelocityinLocalSpace (Variables|Default|GetProjectileMovement) (Math|Vector|MakeVector 0.0 0.0 (Variables|System|GetMissileSpeed)))
  (return))