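; Base HUD Blueprint that provides options menu display and input focus switching, and applies saved settings at startup.
; BeginPlay has BP_GameInstance check graphics, sound and game settings.
; OptionsMenu clears all widgets, then shows an options widget that is created once and cached.
; Focus sets cursor visibility and input mode for game, UI or both, while Back is an empty stub.
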(event Custom|OptionsMenu
  (Viewport|RemoveAllWidgets)
  (Variables|Default|GetW_OptionsMenu
    (:then
      _)
    (:else
      (bind _returnvalue (UserInterface|CreateWidget (Variables|Default|GetOptionsMenuWidget) (Game|Player|GetOwningPlayerController)))
      (bind _output_get (Variables|Default|SetW_OptionsMenu _returnvalue))))
  (UserInterface|Viewport|AddtoViewport _output_get 0))

(event EventBeginPlay
  (bind _asbp_game_instance (System|GetGameInstance))
  ;[1 1 1] Apply initial settings
  (Default|CheckGraphicsSettings _asbp_game_instance)
  (Default|CheckSoundSettings _asbp_game_instance)
  (Default|CheckGameSettings _asbp_game_instance))

(fn ConstructionScript)

(fn Focus
  (params (Focus :type Enum_Focus%20Enum :default "NewEnumerator0"))
  (bind _returnvalue (Game|Player|GetOwningPlayerController))
  (Variables|/Script/Engine.PlayerController|SetbShowMouseCursor (Game|Player|GetOwningPlayerController) (Utilities|Select :Index Focus :NewEnumerator0 true :NewEnumerator1 false :NewEnumerator2 true))
  (switch Utilities|FlowControl|Switch|SwitchonEnum_Focus Focus
    (:NewEnumerator0
      (Input|SetInputModeGameandUI _returnvalue 0 "DoNotLock" true))
    (:NewEnumerator1
      (Input|SetInputModeGameOnly _returnvalue))
    (:NewEnumerator2
      (Input|SetInputModeUIOnly _returnvalue 0 "DoNotLock")))
  (return))

(fn GetGameInstance
  (return (.AsBP%20Game%20Instance (Utilities|Casting|CastToBP_GameInstance (Game|GetGameInstance)))))

(fn Back)